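; Room volume for the FadeRoof tool that fades a room's objects in or out as a group.
; GatherActors runs a debug-drawn Visibility box trace over its Box, rebuilding StaticObject from hit actors implementing BPI_TransparencySetting.
; FadeRoom sends FadeOut or FadeIn interface messages to everything in StaticObject and DynamiqueObject.
; DynamiqueObject is not filled within this Blueprint's graphs.
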(event `Gather Actors`
  (bind _box (`self.Box`))
  (bind _returnvalue (`SceneComponent.K2_GetComponentLocation` _box))
  (`KismetArrayLibrary.Array_Clear` (`self.StaticObject`))
  (bind _outhits (`KismetSystemLibrary.BoxTraceMulti` :`Start` _returnvalue :`End` (+ _returnvalue (0.0 0.0 0.01)) :`HalfSize` (`BoxComponent.GetScaledBoxExtent` _box) :`Orientation` (`SceneComponent.K2_GetComponentRotation` _box) :`TraceChannel` "TraceTypeQuery1" :`DrawDebugType` "ForDuration"))
  (for _array_element _outhits
    (bind (_bblockinghit _binitialoverlap _time _distance _location _impactpoint _normal _impactnormal _physmat _hitactor) (`GameplayStatics.BreakHitResult` _array_element))
    (if (`KismetSystemLibrary.DoesImplementInterface` _hitactor "/Game/GameBank/Blueprints/Tool/FadeRoof/BPI_TransparencySetting.BPI_TransparencySetting_C")
      (`KismetArrayLibrary.Array_Add` (`self.StaticObject`) _hitactor))))

(event `FadeRoom`
  (params (bShouldFade :type Boolean))
  (for _array_element (`self.StaticObject`)
    (if bShouldFade
      (message `/Game/GameBank/Blueprints/Tool/FadeRoof/BPI_TransparencySetting.FadeOut` _array_element)
      (else
        (message `/Game/GameBank/Blueprints/Tool/FadeRoof/BPI_TransparencySetting.FadeIn` _array_element))))
  (for _array_element_2 (`self.DynamiqueObject`)
    (if bShouldFade
      (message `/Game/GameBank/Blueprints/Tool/FadeRoof/BPI_TransparencySetting.FadeOut` _array_element_2)
      (else
        (message `/Game/GameBank/Blueprints/Tool/FadeRoof/BPI_TransparencySetting.FadeIn` _array_element_2)))))

(fn `UserConstructionScript`)