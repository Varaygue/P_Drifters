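; Environment actor that can fade its static mesh out and back in, likely as part of a roof-fading tool.
; BeginPlay creates a dynamic material instance on material slot 0, whose FadeAmount parameter is driven by the Fader timeline.
; FadeOut plays the timeline and makes the mesh ignore the Visibility channel, while Fadein reverses it and restores blocking.
; IsFaded returns the Faded flag, which these graphs never set.
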(event `self.ReceiveBeginPlay`
  (bind _staticmesh (`self.StaticMesh`))
  (bind _returnvalue (`PrimitiveComponent.CreateDynamicMaterialInstance` _staticmesh 0 (`PrimitiveComponent.GetMaterial` _staticmesh 0) "None"))
  (set `self.MI` _returnvalue))

(event `/Game/GameBank/Blueprints/Tool/FadeRoof/BPI_TransparencySetting.FadeOut`
  (`PrimitiveComponent.SetCollisionResponseToChannel` (`self.StaticMesh`) "ECC_Visibility" "ECR_Ignore")
  (bind (_direction _alpha) (`Timeline|Fader` :!label _label)
    (:`Update`
      (`MaterialInstanceDynamic.SetScalarParameterValue` (`self.MI`) "FadeAmount" _alpha))))

(event `/Game/GameBank/Blueprints/Tool/FadeRoof/BPI_TransparencySetting.FadeIn`
  (`PrimitiveComponent.SetCollisionResponseToChannel` (`self.StaticMesh`) "ECC_Visibility" "ECR_Block")
  (goto _label :!via `Reverse`))

(fn `IsFaded`
  (returns (bIsFade :type Boolean))
  (return (`self.bFaded`)))

(fn `UserConstructionScript`)