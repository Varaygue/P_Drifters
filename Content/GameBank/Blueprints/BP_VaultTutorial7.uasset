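; BP_VaultTutorial7 is a one-shot tutorial trigger that shows an input prompt and later hands over to an enemy sequence.
; The first Box overlap, with no filter on the overlapping actor, adds the W_InputTutorial07 widget to the viewport and sets EnableTuto.
; EnemyTutorial, a custom event not called within this graph, runs once to call AssignPoints on EnemyReference, disable player input and remove the widget.
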(event `self.Box.OnComponentBeginOverlap`
  (params (OverlappedComponent :type "PrimitiveComponent Object Reference") (OtherActor :type "Actor Object Reference") (OtherComp :type "PrimitiveComponent Object Reference") (OtherBodyIndex :type Integer) (bFromSweep :type Boolean) (SweepResult :type "HitResult Structure (by ref)"))
  (`/Engine/EditorBlueprintResources/StandardMacros.DoOnce` false
    (:`Completed`
      (bind _returnvalue (`|CreateWidget` "/Game/GameBank/Blueprints/Widgets/W_InputTutorial07.W_InputTutorial07_C"))
      (bind _output_get (set `self.HideTutorial` _returnvalue))
      (`UserWidget.AddToViewport` _output_get 0)
      (set `self.EnableTuto` true))))

(event `EnemyTutorial`
  (`/Engine/EditorBlueprintResources/StandardMacros.DoOnce` false
    (:`Completed`
      (`/Game/GameBank/Blueprints/Characters/AI/BP_EnemyTutorial.AssignPoints` (`self.EnemyReference`))
      (bind _asbp_third_person_character (cast `/Game/GameBank/Blueprints/Characters/Player/Zone/BP_ThirdPersonCharacter` (`GameplayStatics.GetPlayerCharacter` 0)))
      (`self.DisableInput` _asbp_third_person_character null)
      (`Widget.RemoveFromParent` (`self.HideTutorial`)))))

(fn `UserConstructionScript`)