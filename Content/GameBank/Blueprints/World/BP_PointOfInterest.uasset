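; BP_PointOfInterest is a clickable world-map marker showing a zone name over a spinning circle plane.
; Clicking copies its POIData level, image, name and guaranteed resources to BP_PlayerWorld, then calls SelectZone.
; Hovering speeds the spin and loops a timeline pulsing the dynamic material's emissive, reset when the cursor leaves.
; Initialize is empty, and token movement with location saving is unconnected.
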(event `self.ReceiveBeginPlay`
  (bind _poidata_name (break `/Game/GameBank/Blueprints/World/S_PointOfInterests` (`self.POIData`)))
  (`TextRenderComponent.K2_SetText` (`self.TextRender`) (`KismetTextLibrary.Conv_StringToText` _poidata_name))
  (bind _returnvalue (`PrimitiveComponent.CreateDynamicMaterialInstance` (`self.Plane`) 0 "/Game/GameBank/Materials/MaterialVFX/M_Cercle_LVL_Inst.M_Cercle_LVL_Inst" "WorldInstance"))
  (set `self.CurrentMaterialInstance` _returnvalue))

(event `self.ReceiveTick`
  (params (DeltaSeconds :type "Float (single-precision)"))
  (`SceneComponent.K2_AddWorldRotation` (`self.Plane`) (`KismetMathLibrary.MakeRotator` 0.0 0.0 (+ (`self.RotationSpeed`) (* 1.0 DeltaSeconds))) false false))

(event `self.ZoneCollision.OnClicked`
  (params (TouchedComponent :type "PrimitiveComponent Object Reference") (ButtonPressed :type "Key Structure"))
  (bind (_name _leveltoload _guarrantedressourcea _guarantedressourceb _image) (break `/Game/GameBank/Blueprints/World/S_PointOfInterests` (`self.POIData`)))
  (bind _asbp_player_world (cast `/Game/GameBank/Blueprints/Characters/Player/World/BP_PlayerWorld` (`GameplayStatics.GetPlayerCharacter` 0)))
  (set `/Game/GameBank/Blueprints/Characters/Player/World/BP_PlayerWorld.ZoneName` (`KismetStringLibrary.Conv_StringToName` _name) _asbp_player_world)
  (set `/Game/GameBank/Blueprints/Characters/Player/World/BP_PlayerWorld.ZoneToLoad` _leveltoload _asbp_player_world)
  (set `/Game/GameBank/Blueprints/Characters/Player/World/BP_PlayerWorld.ZoneType` _image _asbp_player_world)
  (set `/Game/GameBank/Blueprints/Characters/Player/World/BP_PlayerWorld.ZoneResources1` _guarrantedressourcea _asbp_player_world)
  (set `/Game/GameBank/Blueprints/Characters/Player/World/BP_PlayerWorld.ZoneResources2` _guarantedressourceb _asbp_player_world)
  (`/Game/GameBank/Blueprints/Characters/Player/World/BP_PlayerWorld.SelectZone` _asbp_player_world))

(event `self.ZoneCollision.OnBeginCursorOver`
  (params (TouchedComponent :type "PrimitiveComponent Object Reference"))
  (set `self.RotationSpeed` 3.0)
  (bind (_direction _emissivetrack) (`Timeline|EmissiveBeat` :!via `PlayFromStart` :!label _label)
    (:`Update`
      (`MaterialInstanceDynamic.SetScalarParameterValue` (`self.CurrentMaterialInstance`) "CircleShaderEmissive" _emissivetrack))
    (:`Finished`
      (`KismetSystemLibrary.RetriggerableDelay` 0.15)
      (goto _label :!via `PlayFromStart`))))

(event `self.ZoneCollision.OnEndCursorOver`
  (params (TouchedComponent :type "PrimitiveComponent Object Reference"))
  (`|ExecutionSequence`
    (:`then_0`
      (goto _label :!via `Stop`))
    (:`then_1`
      (set `self.RotationSpeed` 1.0)
      (`MaterialInstanceDynamic.SetScalarParameterValue` (`self.CurrentMaterialInstance`) "CircleShaderEmissive" 0.0))))

(fn `Initialize`
  (params (Row :type "/Game/GameBank/Blueprints/World/S_PointOfInterests Structure")))

(fn `UserConstructionScript`)