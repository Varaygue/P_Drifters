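; BP_PlayerCamp is the camp actor that handles camera moves and an end-of-day lighting transition.
; BeginPlay enables game-and-UI input and stores the camera's starting location.
; EndDay plays a timeline that rotates the level's directional light pitch.
; CameraMovement and Return open Tick-driven gates that ease the camera toward a selected camera or back to the start, each closing after a delay.
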(event `EndDay`
  (bind _returnvalue (`GameplayStatics.GetActorOfClass` "/Script/Engine.DirectionalLight"))
  (bind _output_get (set `self.Light` _returnvalue))
  (bind (_direction _rotationday) (`Timeline|DayEnding`)
    (:`Update`
      (`SceneComponent.K2_SetWorldRotation` (`Actor.RootComponent` _output_get) (`KismetMathLibrary.MakeRotator` 0.0 _rotationday) false false))))

(event `self.ReceiveBeginPlay`
  (`WidgetBlueprintLibrary.SetInputMode_GameAndUIEx` (`GameplayStatics.GetPlayerController` 0) null "DoNotLock" false)
  (set `self.OriginalLoc` (`SceneComponent.K2_GetComponentLocation` (`self.Camera`))))

(event `CameraMovement`
  (goto _label :!via `Open`))

(event `self.ReceiveTick`
  (params (DeltaSeconds :type "Float (single-precision)"))
  (bind _camera (`self.Camera`))
  (`|ExecutionSequence`
    (:`then_0`
      (`/Engine/EditorBlueprintResources/StandardMacros.Gate` true :!label _label
        (:`Exit`
          (`SceneComponent.K2_SetWorldLocation` _camera (`KismetMathLibrary.VInterpTo` (`SceneComponent.K2_GetComponentLocation` (`self.Camera`)) (`SceneComponent.K2_GetComponentLocation` (`self.SelectedCamera`)) DeltaSeconds 2.0) false false)
          (`KismetSystemLibrary.Delay` 2.0)
          (goto _label :!via `Close`))))
    (:`then_1`
      (`/Engine/EditorBlueprintResources/StandardMacros.Gate` true :!label _label_2
        (:`Exit`
          (`SceneComponent.K2_SetWorldLocation` _camera (`KismetMathLibrary.VInterpTo` (`SceneComponent.K2_GetComponentLocation` (`self.Camera`)) (`self.OriginalLoc`) DeltaSeconds 2.0) false false)
          (`KismetSystemLibrary.Delay` 2.0)
          (goto _label_2 :!via `Close`))))))

(event `Return`
  (goto _label_2 :!via `Open`))

(fn `UserConstructionScript`)