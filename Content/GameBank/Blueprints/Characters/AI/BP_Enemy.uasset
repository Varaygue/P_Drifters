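; Enemy AI character that patrols, detects and chases the player, feeding its senses and states to a behavior tree through Blackboard keys.
; Sight of an unhidden player starts a reversible detection timeline that escalates to a faster chase, while hearing sets a target location.
; An attack-range overlap flags the player, including inside hiding spots.
; It also offers toggleable sense debug drawing and briefly shows a tutorial widget when destroyed.
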(event `self.ReceiveDestroyed`
  (`/Engine/EditorBlueprintResources/StandardMacros.DoOnce` false
    (:`Completed`
      (bind _returnvalue (`|CreateWidget` "/Game/GameBank/Blueprints/Widgets/W_InputTutorial08.W_InputTutorial08_C"))
      (`UserWidget.AddToViewport` _returnvalue 0)
      (`KismetSystemLibrary.Delay` 5.0)
      (`Widget.RemoveFromParent` _returnvalue))))

(event `self.ReceiveBeginPlay`
  (bind _output_get (set `self.BlackboardRef` (`AIBlueprintHelperLibrary.GetBlackboard` (`self.GetController`))))
  (if (<= (`KismetArrayLibrary.Array_Length` (`self.PatrolPoints`)) 0)
    (`BlackboardComponent.SetValueAsBool` _output_get "ShouldPatrol" false)))

(event `self.AIPerception.OnTargetPerceptionUpdated`
  (params (Actor :type "Actor Object Reference") (Stimulus :type "AIStimulus Structure"))
  (`self.HandleHearingSense` Stimulus)
  (`self.HandleSightSense` Actor Stimulus))

(event `/Game/GameBank/Blueprints/Characters/AI/BPI_Detection.StartChase`
  (bind _blackboardref (`self.BlackboardRef`))
  (`GameplayStatics.PlaySound2D` "/Game/GameBank/SFX/SoundEffects/Ennemy/SC_Ennemy_Bark_Alert.SC_Ennemy_Bark_Alert" 1.0 1.0 0.0 null null)
  (`BlackboardComponent.SetValueAsBool` _blackboardref "IsChasing" true)
  (`BlackboardComponent.SetValueAsBool` _blackboardref "IsSuspicious" true))

(event `/Game/GameBank/Blueprints/Characters/AI/BPI_Detection.StopChase`
  (bind _blackboardref (`self.BlackboardRef`))
  (`BlackboardComponent.SetValueAsBool` _blackboardref "IsChasing" false)
  (`BlackboardComponent.SetValueAsVector` _blackboardref "TargetLocation" (`self.K2_GetActorLocation` (`GameplayStatics.GetPlayerCharacter` 0))))

(event `/Game/GameBank/Blueprints/Characters/AI/BPI_Detection.StartDetection`
  (params (AI :type "Character Object Reference"))
  (`SceneComponent.SetVisibility` (`self.Widget`) true false)
  (`GameplayStatics.PlaySound2D` "/Game/GameBank/SFX/SoundEffects/Ennemy/SC_Ennemy_Bark_Suspicious.SC_Ennemy_Bark_Suspicious" 1.0 1.0 0.0 null null)
  (`BlackboardComponent.SetValueAsBool` (`self.BlackboardRef`) "IsDetecting" true)
  (bind (_direction _detectionprogress) (`Timeline|Detection` :!label _label)
    (:`Update`
      (bind _output_get (set `self.DetectionProgress` _detectionprogress)))
    (:`Finished`
      (if (!= _output_get 0.0)
        (`/Game/GameBank/Blueprints/Characters/AI/BPI_Detection.StartChase`)
        (set `CharacterMovementComponent.MaxWalkSpeed` 400.0 (`self.CharacterMovement`))
        (`SceneComponent.SetVisibility` (`self.Widget`) false false)))))

(event `/Game/GameBank/Blueprints/Characters/AI/BPI_Detection.StopDetection`
  (`SceneComponent.SetVisibility` (`self.Widget`) false false)
  (`BlackboardComponent.SetValueAsBool` (`self.BlackboardRef`) "IsDetecting" false)
  (goto _label :!via `Reverse`))

(event `self.AttackRange.OnComponentBeginOverlap`
  (params (OverlappedComponent :type "PrimitiveComponent Object Reference") (OtherActor :type "Actor Object Reference") (OtherComp :type "PrimitiveComponent Object Reference") (OtherBodyIndex :type Integer) (bFromSweep :type Boolean) (SweepResult :type "HitResult Structure (by ref)"))
  (cast `/Game/GameBank/Blueprints/Characters/Player/Zone/BP_ThirdPersonCharacter` OtherActor
    (:`then`
      (`BlackboardComponent.SetValueAsBool` (`self.BlackboardRef`) "InAttackRange" true))
    (:`CastFailed`
      (bind _asbp_hiding_spot_base (cast `/Game/GameBank/Blueprints/Ingredients/HidingSpot/BP_HidingSpot_Base` OtherActor))
      (if (`/Game/GameBank/Blueprints/Ingredients/HidingSpot/BP_HidingSpot_Base.IsPlayerInside` _asbp_hiding_spot_base)
        (`BlackboardComponent.SetValueAsBool` (`self.BlackboardRef`) "InAttackRange" true)))))

(event `self.AttackRange.OnComponentEndOverlap`
  (params (OverlappedComponent :type "PrimitiveComponent Object Reference") (OtherActor :type "Actor Object Reference") (OtherComp :type "PrimitiveComponent Object Reference") (OtherBodyIndex :type Integer))
  (cast `/Game/GameBank/Blueprints/Characters/Player/Zone/BP_ThirdPersonCharacter` OtherActor)
  (`BlackboardComponent.SetValueAsBool` (`self.BlackboardRef`) "InAttackRange" false))

(event `self.ReceiveTick`
  (params (DeltaSeconds :type "Float (single-precision)"))
  (bind _returnvalue (`self.K2_GetActorLocation`))
  (`|ExecutionSequence`
    (:`then_0`
      (`/Engine/EditorBlueprintResources/StandardMacros.Gate` true :!label _label_2
        (:`Exit`
          (`KismetSystemLibrary.DrawDebugCircle` _returnvalue 1000.0 12 (struct :`R` 0.029139 :`G` 1.0 :`A` 1.0) 0.0 0.5 (1.0 0.0 0.0) (0.0 1.0 0.0))
          (`KismetSystemLibrary.DrawDebugConeInDegrees` _returnvalue (`self.GetActorForwardVector`) 1000.0 60.0 1.0 12 (struct :`R` 1.0 :`G` 0.038465 :`A` 1.0) 0.0 0.5))))
    (:`then_1`
      (`/Engine/EditorBlueprintResources/StandardMacros.Gate` true :!label _label_3
        (:`Exit`
          (`KismetSystemLibrary.DrawDebugCircle` (`self.K2_GetActorLocation`) 3000.0 12 (struct :`R` 1.0 :`B` 0.846405 :`A` 1.0) 0.0 1.0 (1.0 0.0 0.0) (0.0 1.0 0.0)))))))

(event `ToggleDebugSight`
  (goto _label_2 :!via `Toggle`))

(event `ToggleDebugHearing`
  (goto _label_3 :!via `Toggle`))

(fn `HandleHearingSense`
  (params (Stimulus :type "AIStimulus Structure (by ref)"))
  (bind _returnvalue (`AIPerceptionSystem.GetSenseClassForStimulus` Stimulus))
  (`KismetSystemLibrary.PrintString` (`KismetSystemLibrary.GetClassDisplayName` _returnvalue))
  (if (== _returnvalue "/Script/AIModule.AISense_Hearing")
    (`BlackboardComponent.SetValueAsVector` (`AIBlueprintHelperLibrary.GetBlackboard` null) "TargetLocation" (`.StimulusLocation` (break `AIStimulus` (`local.Stimulus`))))
    (`KismetSystemLibrary.PrintString` "value set")
    (else
      (return))))

(fn `HandleSightSense`
  (params (Object :type "Object Object Reference") (AIStimulus :type "AIStimulus Structure (by ref)"))
  (bind _returnvalue (`AIPerceptionSystem.GetSenseClassForStimulus` AIStimulus))
  (if (== _returnvalue "/Script/AIModule.AISense_Sight")
    (bind _asbp_third_person_character (cast `/Game/GameBank/Blueprints/Characters/Player/Zone/BP_ThirdPersonCharacter` Object))
    (if (and (not (`/Game/GameBank/Blueprints/Characters/Player/Zone/BP_ThirdPersonCharacter.isHiding` _asbp_third_person_character)) (`.bSuccessfullySensed` (break `AIStimulus` AIStimulus)))
      (`BlackboardComponent.SetValueAsObject` (`self.BlackboardRef`) "PlayerRef" (`local.Object`))
      (`/Engine/EditorBlueprintResources/StandardMacros.DoOnce` false :!label _label
        (:`Completed`
          (message `/Game/GameBank/Blueprints/Characters/AI/BPI_Detection.StartDetection` self self)
          (goto _label_2 :!via `Reset`)))
      (else
        (`/Game/GameBank/Blueprints/Characters/AI/BPI_Detection.StopChase`)
        (`/Engine/EditorBlueprintResources/StandardMacros.DoOnce` false :!label _label_2
          (:`Completed`
            (`KismetSystemLibrary.PrintString` "Stop detection")
            (message `/Game/GameBank/Blueprints/Characters/AI/BPI_Detection.StopDetection` self)
            (goto _label :!via `Reset`)))))
    (else
      (return))))

(fn `UpdateWalkSpeed`
  (params (`New Walk Speed` :type "Float (double-precision)"))
  (set `CharacterMovementComponent.MaxWalkSpeed` `New Walk Speed` (`self.CharacterMovement`)))

(fn `UserConstructionScript`)