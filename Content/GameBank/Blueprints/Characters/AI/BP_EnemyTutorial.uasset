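; Scripted AI enemy for the hiding tutorial that walks to a patrol point, then removes itself.
; AssignPoints disables the player's CanOffset, swaps the HUD for the hide widget, then after a delay sets a patrol point and the blackboard's ShouldPatrol flag.
; Tick re-enables player input and destroys the enemy near that point.
; Destroyed restores CanOffset and the HUD and shows the next input tutorial.
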(event `self.ReceiveBeginPlay`)

(event `self.ReceiveTick`
  (params (DeltaSeconds :type "Float (single-precision)"))
  (`parent.ReceiveTick` DeltaSeconds)
  (if (`KismetArrayLibrary.Array_IsNotEmpty` (`self.PatrolPoints`))
    (if (<= (`KismetMathLibrary.VSize` (- (`self.K2_GetActorLocation` (`|GetArrayItem` (`self.PatrolPoints`))) (`self.K2_GetActorLocation`))) 100.0)
      (`/Engine/EditorBlueprintResources/StandardMacros.DoOnce` false
        (:`Completed`
          (bind _asbp_third_person_character (cast `/Game/GameBank/Blueprints/Characters/Player/Zone/BP_ThirdPersonCharacter` (`GameplayStatics.GetPlayerCharacter` 0)))
          (`self.EnableInput` _asbp_third_person_character null)
          (`self.K2_DestroyActor`))))))

(event `AssignPoints`
  (bind _asbp_third_person_character (cast `/Game/GameBank/Blueprints/Characters/Player/Zone/BP_ThirdPersonCharacter` (`GameplayStatics.GetPlayerCharacter` 0)))
  (bind _output_get (set `self.PlayerReference` _asbp_third_person_character))
  (set `/Game/GameBank/Blueprints/Characters/Player/Zone/BP_ThirdPersonCharacter.canOffset` false _output_get)
  (bind _returnvalue (`|CreateWidget` "/Game/GameBank/HUD/Widgets/Player/Zone/Tutorials/WBP_HideTutorial.WBP_HideTutorial_C"))
  (bind _output_get_2 (set `self.TutorialHide` _returnvalue))
  (`UserWidget.AddToViewport` _output_get_2 0)
  (bind _foundwidgets (`WidgetBlueprintLibrary.GetAllWidgetsOfClass` "/Game/GameBank/Blueprints/Widgets/W_PlayerHUD.W_PlayerHUD_C"))
  (`Widget.RemoveFromParent` (`|GetArrayItem` _foundwidgets))
  (`KismetSystemLibrary.Delay` 2.0)
  (bind _returnvalue_2 (`GameplayStatics.GetActorOfClass` "/Game/GameBank/Blueprints/Characters/AI/BP_PatrolPoint.BP_PatrolPoint_C"))
  (`KismetArrayLibrary.Array_Add` (`self.PatrolPoints`) _returnvalue_2)
  (bind _output_get_3 (set `self.BlackboardRef` (`AIBlueprintHelperLibrary.GetBlackboard` (`self.GetController`))))
  (if (<= (`KismetArrayLibrary.Array_Length` (`self.PatrolPoints`)) 1)
    (`BlackboardComponent.SetValueAsBool` _output_get_3 "ShouldPatrol" true)
    (`KismetSystemLibrary.PrintString` "IsPatrolling")))

(event `self.ReceiveDestroyed`
  (bind _returnvalue (`GameplayStatics.GetActorOfClass` "/Game/GameBank/Blueprints/Characters/Player/Zone/BP_ThirdPersonCharacter.BP_ThirdPersonCharacter_C"))
  (set `/Game/GameBank/Blueprints/Characters/Player/Zone/BP_ThirdPersonCharacter.canOffset` true _returnvalue)
  (`Widget.RemoveFromParent` (`self.TutorialHide`))
  (bind _returnvalue_2 (`|CreateWidget` "/Game/GameBank/Blueprints/Widgets/W_PlayerHUD.W_PlayerHUD_C"))
  (`UserWidget.AddToViewport` _returnvalue_2 1)
  (bind _returnvalue_3 (`|CreateWidget` "/Game/GameBank/Blueprints/Widgets/W_InputTutorial08.W_InputTutorial08_C"))
  (`UserWidget.AddToViewport` _returnvalue_3 0))

(fn `UserConstructionScript`
  (`parent.UserConstructionScript`))