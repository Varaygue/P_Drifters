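; Player actor for the camp phase, managing food, health, hope, protection and tech alongside the camp UI, menus and debug tools.
; Loads resources from the game instance; consumption drains food and health, or during a crisis rolls against hope for recovery or game over.
; Gated Tick blends views between building or main cameras, while events handle fade-timed construction, day-end sun rotation and the protection-based win check.
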(event Custom|CameraMovement
  (Utilities|FlowControl|Gate true) ; enters at Open
)

(event Custom|Return
  (Utilities|FlowControl|Gate true) ; enters at Open
)

(event Custom|EndDay
  (bind _returnvalue (Actor|GetActorOfClass "/Script/Engine.DirectionalLight"))
  (bind _output_get (Variables|Default|SetLight _returnvalue))
  (bind _rotationday (Timeline|DayEnding Play)
    (:Update
      (Transformation|SetWorldRotation (Variables|/Script/Engine.Actor|GetRootComponent _output_get) (Math|Rotator|MakeRotator -41.0 _rotationday -42.0) false false))))

(event Custom|Build
  (bind _returnvalue (UserInterface|CreateWidget "/Game/GameBank/HUD/Widgets/Player/Camp/WBP_BuildingFade.WBP_BuildingFade_C"))
  (bind _output_get (Variables|Default|SetBuildingProcess _returnvalue))
  (UserInterface|Viewport|AddtoViewport _returnvalue 0)
  (Class|UserWidget|BindtoAnimationFinished (Variables|Default|GetBuildingProcess) (Variables|/Game/GameBank/HUD/Widgets/Player/Camp/WBP_BuildingFade.WBP_BuildingFade_C|GetBuildingFade (Variables|Default|GetBuildingProcess)) (delegate Custom|BuildingDone)))

(event Custom|Consommation
  (if (Variables|/Game/GameBank/Blueprints/GameInstance/GI_GameInstance.GI_GameInstance_C|GetCrisisOngoing (Variables|Default|GetGameInstance))
    (bind _success (CallFunction|RollHope))
    (Utilities|FlowControl|Delay 5.0)
    (if _success
      (bind _returnvalue (UserInterface|CreateWidget "/Game/GameBank/HUD/Widgets/Player/Camp/WBP_HopeSuccess.WBP_HopeSuccess_C"))
      (UserInterface|Viewport|AddtoViewport _returnvalue 3)
      (Utilities|FlowControl|Delay 5.0)
      (Widget|RemovefromParent _returnvalue)
      (CallFunction|RestoreRessources)
      (else
        (CallFunction|GameOver)))
    (else
      (CallFunction|DecreaseResources "NewEnumerator3" true)
      (CallFunction|DecreaseResources "NewEnumerator0" true))))

(event Custom|DisableTutorial
  (bind _campwidget (Variables|Default|GetCampWidget))
  (Widget|RemovefromParent (Variables|/Game/GameBank/HUD/Widgets/Player/Camp/WBP_CampInterface.WBP_CampInterface_C|GetCampTutorialWidget _campwidget))
  (Widget|SetIsEnabled (Variables|/Game/GameBank/HUD/Widgets/Player/Camp/WBP_CampInterface.WBP_CampInterface_C|GetCampMainButton _campwidget) true))

(event Custom|BuildingDone
  (Default|SetGameInstanceBuilt (Variables|Buildings|GetFocusedBuilding) (Variables|Default|GetGameInstance) true)
  (Widget|RemovefromParent (Variables|Default|GetBuildingProcess)))

(event Custom|ChangeBuilding
  (Default|SetBuildingMeshState (Variables|Buildings|GetFocusedBuilding) true))

(event Custom|CheckGameEnd
  (Utilities|FlowControl|DoOnce false
    (:Completed
      (if (>= (Variables|Default|GetProtCurrent) 8e+01)
        (bind _returnvalue (UserInterface|CreateWidget "/Game/GameBank/HUD/Widgets/Player/Camp/WBP_WinScreen.WBP_WinScreen_C"))
        (UserInterface|Viewport|AddtoViewport _returnvalue 5)
        (else
          (bind _returnvalue_2 (UserInterface|CreateWidget "/Game/GameBank/HUD/WBP_GameOver.WBP_GameOver_C"))
          (UserInterface|Viewport|AddtoViewport _returnvalue_2 5))))))

(event Input|EnhancedActionEvents|EnhancedInputActionIA_StartMenu
  (params (ActionValue :type Boolean) (ElapsedSeconds :type Float%20%28double-precision%29) (TriggeredSeconds :type Float%20%28double-precision%29) (InputAction :type Input%20Action%20Object%20Reference :default "/Game/GameBank/Input/Actions/IA_StartMenu.IA_StartMenu"))
  ;[1 1 1] Start Menu
  (Utilities|FlowControl|FlipFlop
    (:A
      (bind _returnvalue (UserInterface|CreateWidget "/Game/GameBank/Blueprints/Widgets/W_EscapeMenu.W_EscapeMenu_C"))
      (bind _output_get (Variables|Default|SetEscapeMenu _returnvalue))
      (UserInterface|Viewport|AddtoViewport _output_get 0)
      (Game|SetGamePaused true))
    (:B
      (Widget|RemovefromParent (Variables|Default|GetEscapeMenu))
      (Variables|Default|SetEscapeMenu (Variables|Default|GetEscapeMenu))
      (Game|SetGamePaused false))))

(event EventBeginPlay
  (bind _outactors (Actor|GetAllActorsOfClass "/Script/Engine.CameraActor"))
  (for _array_element _outactors
    (if (Utilities|Enum|Equal(Enum) (Utilities|GetDisplayName _array_element) "MainCamera")
      (Variables|Default|SetBaseCamera _array_element)
      (bind _asgi_game_instance (Utilities|Casting|CastToGI_GameInstance (Game|GetGameInstance)))
      (bind _output_get (Variables|Default|SetGameInstance _asgi_game_instance))
      (Variables|Default|SetLastFood (Variables|/Game/GameBank/Blueprints/GameInstance/GI_GameInstance.GI_GameInstance_C|GetCachedFood _output_get))
      (Variables|Default|SetLastHealth (Variables|/Game/GameBank/Blueprints/GameInstance/GI_GameInstance.GI_GameInstance_C|GetCachedHealth _output_get))
      (Variables|Default|SetLastHope (Variables|/Game/GameBank/Blueprints/GameInstance/GI_GameInstance.GI_GameInstance_C|GetCachedHope _output_get))
      (Variables|Default|SetLastProt (Variables|/Game/GameBank/Blueprints/GameInstance/GI_GameInstance.GI_GameInstance_C|GetCachedProtection _output_get))
      (bind _returnvalue (UserInterface|CreateWidget "/Game/GameBank/HUD/Widgets/Player/Camp/WBP_CampInterface.WBP_CampInterface_C"))
      (bind _output_get_2 (Variables|Default|SetCampWidget _returnvalue))
      (UserInterface|Viewport|AddtoViewport _output_get_2 0)
      (CallFunction|Initialize)
      (bind _outactors_2 (Actor|GetAllActorsOfClass "/Script/Engine.CameraActor"))
      (Variables|Default|SetActiveCamera (Utilities|Array|Get(acopy) _outactors_2 3))
      (if (Variables|/Game/GameBank/Blueprints/GameInstance/GI_GameInstance.GI_GameInstance_C|GetFirstTimeInCamp (Variables|Default|GetGameInstance))
        (bind _returnvalue_2 (UserInterface|CreateWidget "/Game/GameBank/HUD/Widgets/Player/Camp/Tutorial/WBP_CampTutorial01.WBP_CampTutorial01_C"))
        (bind _output_get_3 (Variables|Default|SetCampTutorial _returnvalue_2))
        (UserInterface|Viewport|AddtoViewport _output_get_3 1)))))

(event EventTick
  (params (DeltaSeconds :type Float%20%28single-precision%29))
  (Variables|Default|SetDelta%20Seconds DeltaSeconds)
  (Utilities|FlowControl|Sequence
    (:then_0
      (Utilities|FlowControl|Gate true :!label _label
        (:Exit
          (Game|Player|SetViewTargetwithBlend (Game|GetPlayerController 0) (Variables|Default|GetSelectedCamera) 1.0 "VTBlend_Linear" 0.0 false)
          (Utilities|FlowControl|Delay 2.0)
          (goto _label Close))))
    (:then_1
      (Utilities|FlowControl|Gate true :!label _label_2
        (:Exit
          (Game|Player|SetViewTargetwithBlend (Game|GetPlayerController 0) (Variables|Default|GetBaseCamera) 1.0 "VTBlend_Cubic" 0.0 false)
          (Utilities|FlowControl|Delay 2.0)
          (goto _label_2 Close))))))

(event Input|KeyboardEvents|DebugKeyK
  (params (Key :type Key%20Structure :default "None") (ActionValue :type Input%20Action%20Value%20Structure))
  (:Pressed
    (Default|ResetGameInstance (Variables|Default|GetGameInstance))
    (CallFunction|Initialize)))

(event Input|KeyboardEvents|²
  (params (Key :type Key%20Structure :default "None"))
  (:Pressed
    (Utilities|FlowControl|FlipFlop
      (:A
        (bind _returnvalue (UserInterface|CreateWidget "/Game/GameBank/HUD/Widgets/Player/Camp/Debug/WBP_CampDebug.WBP_CampDebug_C"))
        (bind _output_get (Variables|Default|SetCampDebug _returnvalue))
        (UserInterface|Viewport|AddtoViewport _output_get 2))
      (:B
        (Widget|RemovefromParent (Variables|Default|GetCampDebug))))))

(event Input|KeyboardEvents|Escape
  (params (Key :type Key%20Structure :default "None"))
  (:Pressed
    (Utilities|FlowControl|FlipFlop
      (:A
        (bind _returnvalue (UserInterface|CreateWidget "/Game/GameBank/Blueprints/Widgets/W_EscapeMenu.W_EscapeMenu_C"))
        (bind _output_get (Variables|Default|SetMenuEchap _returnvalue))
        (UserInterface|Viewport|AddtoViewport _output_get 0))
      (:B
        (Widget|RemovefromParent (Variables|Default|GetMenuEchap))))))

(fn ConstructionScript)

(fn IncreaseResources
  (params (Type :type E_ItemTypes%20Enum :default "NewEnumerator3") (TargetValue :type Float%20%28double-precision%29) (Multiplier :type Float%20%28double-precision%29))
  (bind _gameinstance (Variables|Default|GetGameInstance))
  (if (not (> TargetValue 0.0))
    ;[1 1 1] With modifiers
    (switch Utilities|FlowControl|Switch|SwitchonE_ItemTypes Type
      (:NewEnumerator3
        (if (Variables|Buildings|GetCanteenBuilt)
          (bind _output_get (Variables|Default|SetFoodCurrent (Math|Float|Clamp(Float) (+ (Variables|Default|GetFoodCurrent) (- (* (Variables|/Game/GameBank/Blueprints/GameInstance/GI_GameInstance.GI_GameInstance_C|GetConsommationValue (Variables|Default|GetGameInstance)) Multiplier) 1e+01)) 0.0 1e+02)))
          (Variables|/Game/GameBank/Blueprints/GameInstance/GI_GameInstance.GI_GameInstance_C|SetFoodValue _gameinstance _output_get)
          (else
            (bind _output_get_2 (Variables|Default|SetFoodCurrent (Math|Float|Clamp(Float) (+ (Variables|Default|GetFoodCurrent) (* (Variables|/Game/GameBank/Blueprints/GameInstance/GI_GameInstance.GI_GameInstance_C|GetConsommationValue (Variables|Default|GetGameInstance)) Multiplier)) 0.0 1e+02)))
            (Variables|/Game/GameBank/Blueprints/GameInstance/GI_GameInstance.GI_GameInstance_C|SetFoodValue _gameinstance _output_get_2))))
      (:NewEnumerator0
        (bind _output_get_3 (Variables|Default|SetHealthCurrent (Math|Float|Clamp(Float) (+ (Variables|Default|GetHealthCurrent) (* (Variables|/Game/GameBank/Blueprints/GameInstance/GI_GameInstance.GI_GameInstance_C|GetConsommationValue (Variables|Default|GetGameInstance)) Multiplier)) 0.0 1e+02)))
        (Variables|/Game/GameBank/Blueprints/GameInstance/GI_GameInstance.GI_GameInstance_C|SetHealthValue _gameinstance _output_get_3))
      (:NewEnumerator1
        (bind _output_get_4 (Variables|Default|SetHopeCurrent (Math|Float|Clamp(Float) (+ (Variables|Default|GetHopeCurrent) (* (Variables|/Game/GameBank/Blueprints/GameInstance/GI_GameInstance.GI_GameInstance_C|GetConsommationValue (Variables|Default|GetGameInstance)) Multiplier)) 0.0 1e+02)))
        (Variables|/Game/GameBank/Blueprints/GameInstance/GI_GameInstance.GI_GameInstance_C|SetHopeValue _gameinstance _output_get_4))
      (:NewEnumerator2
        (bind _output_get_5 (Variables|Default|SetProtCurrent (Math|Float|Clamp(Float) (+ (Variables|Default|GetProtCurrent) (* (Variables|/Game/GameBank/Blueprints/GameInstance/GI_GameInstance.GI_GameInstance_C|GetConsommationValue (Variables|Default|GetGameInstance)) Multiplier)) 0.0 1e+02)))
        (Variables|/Game/GameBank/Blueprints/GameInstance/GI_GameInstance.GI_GameInstance_C|SetProtectionValue _gameinstance _output_get_5))
      (:NewEnumerator5
        (bind _output_get_6 (Variables|Default|SetTechCurrent (Math|Float|Clamp(Float) (+ (Variables|Default|GetTechCurrent) 1.0) 0.0 1e+02)))
        (Variables|/Game/GameBank/Blueprints/GameInstance/GI_GameInstance.GI_GameInstance_C|SetTechValue _gameinstance _output_get_6)))
    (else
      ;[1 1 1] Without Modifiers
      (switch Utilities|FlowControl|Switch|SwitchonE_ItemTypes Type
        (:NewEnumerator3
          (Variables|Default|SetFoodCurrent (Math|Float|Lerp (Variables|Default|GetFoodCurrent) (Math|Float|Clamp(Float) (+ (Variables|Default|GetFoodCurrent) TargetValue) 0.0 1e+02) 1.0)))
        (:NewEnumerator0
          (Variables|Default|SetHealthCurrent (Math|Float|Lerp (Variables|Default|GetHealthCurrent) (Math|Float|Clamp(Float) (+ (Variables|Default|GetHealthCurrent) TargetValue) 0.0 1e+02) 1.0)))
        (:NewEnumerator1
          (Variables|Default|SetHopeCurrent (Math|Float|Clamp(Float) (+ (Variables|Default|GetHopeCurrent) TargetValue) 0.0 1e+02)))
        (:NewEnumerator2
          (Variables|Default|SetProtCurrent (Math|Float|Clamp(Float) (+ (Variables|Default|GetProtCurrent) TargetValue) 0.0 1e+02)))
        (:NewEnumerator5
          (bind _output_get_7 (Variables|Default|SetTechCurrent (Math|Float|Clamp(Float) TargetValue 0.0 1e+02)))
          (Development|PrintString (Utilities|String|ToString(Float) _output_get_7) true true "(R=1.000000,G=0.000000,B=0.022307,A=1.000000)"))))))

(fn DecreaseResources
  (params (Type :type E_ItemTypes%20Enum :default "NewEnumerator3") (ApplyModifiers :type Boolean))
  (if ApplyModifiers
    ;[1 1 1] With modifiers
    (switch Utilities|FlowControl|Switch|SwitchonE_ItemTypes Type
      (:NewEnumerator3
        (if (Variables|Buildings|GetCanteenBuilt)
          (Variables|Default|SetFoodCurrent (Math|Float|Clamp(Float) (- (Variables|Default|GetFoodCurrent) (- (Variables|/Game/GameBank/Blueprints/GameInstance/GI_GameInstance.GI_GameInstance_C|GetConsommationValue (Variables|Default|GetGameInstance)) 1e+01)) 0.0 1e+02))
          (else
            (Variables|Default|SetFoodCurrent (Math|Float|Clamp(Float) (- (Variables|Default|GetFoodCurrent) (Variables|/Game/GameBank/Blueprints/GameInstance/GI_GameInstance.GI_GameInstance_C|GetConsommationValue (Variables|Default|GetGameInstance))) 0.0 1e+02)))))
      (:NewEnumerator0
        (Variables|Default|SetHealthCurrent (Math|Float|Clamp(Float) (- (Variables|Default|GetHealthCurrent) (Variables|/Game/GameBank/Blueprints/GameInstance/GI_GameInstance.GI_GameInstance_C|GetConsommationValue (Variables|Default|GetGameInstance))) 0.0 1e+02)))
      (:NewEnumerator1
        (Variables|Default|SetHopeCurrent (Math|Float|Clamp(Float) (- (Variables|Default|GetHopeCurrent) (Variables|/Game/GameBank/Blueprints/GameInstance/GI_GameInstance.GI_GameInstance_C|GetConsommationValue (Variables|Default|GetGameInstance))) 0.0 1e+02)))
      (:NewEnumerator2
        (Variables|Default|SetProtCurrent (Math|Float|Clamp(Float) (- (Variables|Default|GetProtCurrent) (Variables|/Game/GameBank/Blueprints/GameInstance/GI_GameInstance.GI_GameInstance_C|GetConsommationValue (Variables|Default|GetGameInstance))) 0.0 1e+02)))
      (:NewEnumerator5
        (Variables|Default|SetTechCurrent (Math|Float|Clamp(Float) (- (Variables|Default|GetTechCurrent) 1.0) 0.0 1e+02))))
    (else
      ;[1 1 1] Without Modifiers
      (switch Utilities|FlowControl|Switch|SwitchonE_ItemTypes Type
        (:NewEnumerator3
          (Variables|Default|SetFoodCurrent (Math|Float|Clamp(Float) (- (Variables|Default|GetFoodCurrent) (Variables|/Game/GameBank/Blueprints/GameInstance/GI_GameInstance.GI_GameInstance_C|GetConsommationValue (Variables|Default|GetGameInstance))) 0.0 1e+02)))
        (:NewEnumerator0
          (Variables|Default|SetHealthCurrent (Math|Float|Clamp(Float) (- (Variables|Default|GetHealthCurrent) (Variables|/Game/GameBank/Blueprints/GameInstance/GI_GameInstance.GI_GameInstance_C|GetConsommationValue (Variables|Default|GetGameInstance))) 0.0 1e+02)))
        (:NewEnumerator1
          (Variables|Default|SetHopeCurrent (Math|Float|Clamp(Float) (- (Variables|Default|GetHopeCurrent) (Variables|/Game/GameBank/Blueprints/GameInstance/GI_GameInstance.GI_GameInstance_C|GetConsommationValue (Variables|Default|GetGameInstance))) 0.0 1e+02)))
        (:NewEnumerator2
          (Variables|Default|SetProtCurrent (Math|Float|Clamp(Float) (- (Variables|Default|GetProtCurrent) (Variables|/Game/GameBank/Blueprints/GameInstance/GI_GameInstance.GI_GameInstance_C|GetConsommationValue (Variables|Default|GetGameInstance))) 0.0 1e+02)))
        (:NewEnumerator5
          (Variables|Default|SetTechCurrent (Math|Float|Clamp(Float) (- (Variables|Default|GetTechCurrent) 1.0) 0.0 1e+02)))))))

(fn RollHope
  (bind _output_get (LocalVariables|SetRollValue (Math|Random|RandomIntegerinRange 0 100)))
  (bind _returnvalue (UserInterface|CreateWidget "/Game/GameBank/HUD/Widgets/Player/Camp/WBP_HopeRoll.WBP_HopeRoll_C" 0 _output_get))
  (UserInterface|Viewport|AddtoViewport _returnvalue 3)
  (if (< _output_get (Variables|Default|GetHopeCurrent))
    (CallFunction|DecreaseResources "NewEnumerator1" false)
    (return true)
    (else
      (return false))))

(fn GameOver
  (Variables|Default|SetIsGameOver true)
  (bind _returnvalue (UserInterface|CreateWidget "/Game/GameBank/HUD/WBP_GameOver.WBP_GameOver_C"))
  (UserInterface|Viewport|AddtoViewport _returnvalue 0)
  (Input|SetInputModeUIOnly (Game|GetPlayerController 0) _returnvalue "DoNotLock" false))

(fn RestoreRessources
  (Utilities|FlowControl|Sequence
    (:then_0
      (if (<= (Variables|Default|GetFoodCurrent) (Variables|/Game/GameBank/Blueprints/GameInstance/GI_GameInstance.GI_GameInstance_C|GetCrisisTreshold (Variables|Default|GetGameInstance)))
        (CallFunction|IncreaseResources "NewEnumerator3" (Variables|/Game/GameBank/Blueprints/GameInstance/GI_GameInstance.GI_GameInstance_C|GetCrisisTreshold (Variables|Default|GetGameInstance)) 1.0)))
    (:then_1
      (if (<= (Variables|Default|GetHealthCurrent) (Variables|/Game/GameBank/Blueprints/GameInstance/GI_GameInstance.GI_GameInstance_C|GetCrisisTreshold (Variables|Default|GetGameInstance)))
        (CallFunction|IncreaseResources "NewEnumerator0" (Variables|/Game/GameBank/Blueprints/GameInstance/GI_GameInstance.GI_GameInstance_C|GetCrisisTreshold (Variables|Default|GetGameInstance)) 1.0)))
    (:then_2
      (Variables|/Game/GameBank/Blueprints/GameInstance/GI_GameInstance.GI_GameInstance_C|SetCrisisOngoing (Variables|Default|GetGameInstance) false))))

(fn UpdateRessources
  (bind _gameinstance (Variables|Default|GetGameInstance))
  (bind _cachedtech (Variables|/Game/GameBank/Blueprints/GameInstance/GI_GameInstance.GI_GameInstance_C|GetCachedTech _gameinstance))
  (Variables|Default|SetFoodCurrent (+ (Variables|Default|GetFoodCurrent) (Variables|/Game/GameBank/Blueprints/GameInstance/GI_GameInstance.GI_GameInstance_C|GetCachedFood (Variables|Default|GetGameInstance))))
  (Variables|Default|SetHealthCurrent (+ (Variables|Default|GetHealthCurrent) (Variables|/Game/GameBank/Blueprints/GameInstance/GI_GameInstance.GI_GameInstance_C|GetCachedHealth (Variables|Default|GetGameInstance))))
  (Variables|Default|SetHopeCurrent (+ (Variables|Default|GetHopeCurrent) (Variables|/Game/GameBank/Blueprints/GameInstance/GI_GameInstance.GI_GameInstance_C|GetCachedHope (Variables|Default|GetGameInstance))))
  (Variables|Default|SetProtCurrent (+ (Variables|Default|GetProtCurrent) (Variables|/Game/GameBank/Blueprints/GameInstance/GI_GameInstance.GI_GameInstance_C|GetCachedProtection (Variables|Default|GetGameInstance))))
  (Development|PrintString (Utilities|String|ToString(Float) _cachedtech) true true "(R=1.000000,G=0.000000,B=0.056522,A=1.000000)" 2e+01)
  (Development|PrintString (Utilities|String|ToString(Float) (Variables|Default|GetTechCurrent)) true true "(R=0.054246,G=1.000000,B=0.000000,A=1.000000)" 2e+01)
  (Development|PrintString (Utilities|String|ToString(Float) (+ (Variables|Default|GetTechCurrent) _cachedtech)) true true "(R=1.000000,G=0.535514,B=0.000000,A=1.000000)" 2e+01)
  (bind _output_get (Variables|Default|SetTechCurrent (+ (Variables|Default|GetTechCurrent) _cachedtech)))
  (Development|PrintString (Utilities|String|ToString(Float) _output_get) true true "(R=0.461308,G=0.000000,B=1.000000,A=1.000000)" 2e+01))

(fn Initialize
  (bind _gameinstance (Variables|Default|GetGameInstance))
  (Variables|Default|SetFoodCurrent (Variables|/Game/GameBank/Blueprints/GameInstance/GI_GameInstance.GI_GameInstance_C|GetFoodValue _gameinstance))
  (Variables|Default|SetHealthCurrent (Variables|/Game/GameBank/Blueprints/GameInstance/GI_GameInstance.GI_GameInstance_C|GetHealthValue _gameinstance))
  (Variables|Default|SetHopeCurrent (Variables|/Game/GameBank/Blueprints/GameInstance/GI_GameInstance.GI_GameInstance_C|GetHopeValue _gameinstance))
  (Variables|Default|SetProtCurrent (Variables|/Game/GameBank/Blueprints/GameInstance/GI_GameInstance.GI_GameInstance_C|GetProtectionValue _gameinstance))
  (Variables|Default|SetTechCurrent (Variables|/Game/GameBank/Blueprints/GameInstance/GI_GameInstance.GI_GameInstance_C|GetTechValue _gameinstance)))

(fn SetActiveBuilding
  (params (Building :type BP%20Buildings%20Object%20Reference)))