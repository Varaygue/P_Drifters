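; Player Blueprint for the world map, which sets up the HUD and randomizes visible points of interest.
; BeginPlay fades in, sets the current location to Camp, hides every unlocked BP_PointOfInterest and, unless WorldLocked, re-shows up to MaxPOI random picks, possibly repeated.
; SelectZone replaces the zone info widget with the zone's name, image and loot types.
; Mouse-wheel handlers are inert, and older spawning, movement and tutorial logic is disconnected.
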(event `Key|MouseScrollUp`
  (params (Key :type "Key Structure"))
  (:`Pressed`
    (if (and (< 0.0 -100.0) (> 0.0 100.0))
      _)))

(event `Key|MouseScrollDown`
  (params (Key :type "Key Structure"))
  (:`Pressed`
    (if (and (> 0.0 -2000.0) (< 0.0 2000.0))
      _)))

(event `self.ReceiveBeginPlay`
  (bind _returnvalue (`|CreateWidget` "/Game/GameBank/HUD/Widgets/Player/Zone/Extract/WBP_FadeOut.WBP_FadeOut_C"))
  (`UserWidget.AddToViewport` _returnvalue 0)
  (`UserWidget.PlayAnimation` _returnvalue (`/Game/GameBank/HUD/Widgets/Player/Zone/Extract/WBP_FadeOut.FadeAnim` _returnvalue) 0.0 1 "Reverse" 1.0 false)
  (`|ExecutionSequence`
    (:`then_0`
      (`KismetArrayLibrary.Array_Clear` (`self.ZonePositions`))
      (set `self.CurrentLocation` (make `/Game/GameBank/Blueprints/World/S_PointOfInterests` "Camp" "Gym_Camp" "NewEnumerator4" "NewEnumerator4" "/Game/GameBank/Texture/bandage.bandage" null))
      (`|ExecutionSequence`
        (:`then_0`
          (bind _returnvalue_2 (`|CreateWidget` "/Game/GameBank/Blueprints/Widgets/World/W_WorldHUD.W_WorldHUD_C"))
          (bind _output_get (set `self.HUDRef` _returnvalue_2))
          (`UserWidget.AddToViewport` _output_get 0)
          (bind _asgi_game_instance (cast `/Game/GameBank/Blueprints/GameInstance/GI_GameInstance` (`GameplayStatics.GetGameInstance`)))
          (set `self.GameInstance` _asgi_game_instance))
        (:`then_1`
          (bind _levelpool (`self.HidePoi`))
          (if (not (`self.WorldLocked`))
            (`self.CreateRandomPoints` _levelpool)))))))

(event `SelectZone`
  (bind _infowidget (`self.InfoWidget`)
    (:`then`
      (`Widget.RemoveFromParent` _infowidget))
    (:`else`
      _))
  (bind _returnvalue (`|CreateWidget` "/Game/GameBank/HUD/Widgets/Player/World/WBP_ZoneInfo.WBP_ZoneInfo_C"))
  (bind _output_get (set `self.InfoWidget` _returnvalue))
  (`/Game/GameBank/HUD/Widgets/Player/World/WBP_ZoneInfo.SetZoneLootImage` _output_get (`self.ZoneResources1`) (`self.ZoneResources2`))
  (`UserWidget.AddToViewport` _output_get 0)
  (set `TextBlock.Text` (`KismetTextLibrary.Conv_NameToText` (`self.ZoneName`)) (`/Game/GameBank/HUD/Widgets/Player/World/WBP_ZoneInfo.ZoneName` _output_get))
  (`Image.SetBrushFromTexture` (`/Game/GameBank/HUD/Widgets/Player/World/WBP_ZoneInfo.ZoneImage` _output_get) (`self.ZoneType`) false))

(fn `CreateRandomPoints`
  (params (LevelPool :type "Array of /Game/GameBank/Blueprints/World/BP_PointOfInterest Object Reference"))
  (for _ (range 1 (+ (`self.MaxPOI`) 1))
    (`SceneComponent.SetVisibility` (`/Game/GameBank/Blueprints/World/BP_PointOfInterest.Scene` (`KismetArrayLibrary.Array_Random` LevelPool)) true true)))

(fn `GetNodeLockedPoints`
  (returns (LockedNodes :type "Array of /Game/GameBank/Blueprints/World/BP_PointOfInterest Object Reference") (Numbers :type Integer))
  (locals (`NodeLocked (local)` :type "Array of /Game/GameBank/Blueprints/World/BP_PointOfInterest Object Reference"))
  (bind _zonepositions (`self.ZonePositions`))
  (bind _nodelocked__local_ (`local.NodeLocked (local)`))
  (if (not (<= (`KismetArrayLibrary.Array_Length` _zonepositions) 0))
    (for _array_element _zonepositions
      (if (`/Game/GameBank/Blueprints/World/BP_PointOfInterest.Locked` _array_element)
        (`KismetArrayLibrary.Array_Add` (`local.NodeLocked (local)`) _array_element)))
    (return _nodelocked__local_ (`KismetArrayLibrary.Array_Length` _nodelocked__local_))))

(fn `GetRandomRow`
  (params (RowNames :type "Array of Name (by ref)") (Quantity :type Integer))
  (returns (`Out Rows` :type "Array of /Game/GameBank/Blueprints/World/S_PointOfInterests Structure"))
  (locals (`RowsFound (local)` :type "Array of /Game/GameBank/Blueprints/World/S_PointOfInterests Structure"))
  (`KismetArrayLibrary.Array_Shuffle` RowNames)
  (for _index (range Quantity)
    (bind _returnvalue (`|GetDataTableRow` "/Game/GameBank/Blueprints/World/S_PoITable.S_PoITable" (`|GetArrayItem` RowNames _index))
      (:`then`
        (`KismetArrayLibrary.Array_Add` (`local.RowsFound (local)`) _returnvalue))))
  (return (`local.RowsFound (local)`)))

(fn `HidePoi`
  (returns (LevelPool :type "Array of /Game/GameBank/Blueprints/World/BP_PointOfInterest Object Reference"))
  (locals (`ZoneLevels (local)` :type "Array of /Game/GameBank/Blueprints/World/BP_PointOfInterest Object Reference"))
  (bind _outactors (`GameplayStatics.GetAllActorsOfClass` "/Game/GameBank/Blueprints/World/BP_PointOfInterest.BP_PointOfInterest_C"))
  (for _array_element _outactors
    (if (not (`/Game/GameBank/Blueprints/World/BP_PointOfInterest.Locked` _array_element))
      (`SceneComponent.SetVisibility` (`/Game/GameBank/Blueprints/World/BP_PointOfInterest.Scene` _array_element) false true)
      (`KismetArrayLibrary.Array_Add` (`local.ZoneLevels (local)`) _array_element)))
  (return (`local.ZoneLevels (local)`)))

(fn `UserConstructionScript`)