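; BP_CameraZone is a placeable box volume that defines rectangular camera bounds, judging by its name and its GetCameraBounds function.
; The construction script sizes the Box component from the Size and Height variables.
; GetCameraBounds returns 2D Min and Max corners as the actor location minus and plus Size, ignoring rotation and Z.
; Its event graph holds no active logic.
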(fn `GetCameraBounds`
  (returns (Min :type "Vector2D Structure") (Max :type "Vector2D Structure"))
  (bind _returnvalue (`self.K2_GetActorLocation`))
  (bind (_x _y) (`KismetMathLibrary.BreakVector2D` (`self.Size`)))
  (bind _returnvalue_2 (`KismetMathLibrary.MakeVector` _x _y))
  (return (`KismetMathLibrary.MakeVector2D` (.x (- _returnvalue _returnvalue_2)) (.y (- _returnvalue _returnvalue_2))) (`KismetMathLibrary.MakeVector2D` (.x (+ _returnvalue _returnvalue_2)) (.y (+ _returnvalue _returnvalue_2)))))

(fn `UserConstructionScript`
  (bind (_x _y) (`KismetMathLibrary.BreakVector2D` (`self.Size`)))
  (`BoxComponent.SetBoxExtent` (`self.Box`) (`KismetMathLibrary.MakeVector` _x _y (`self.Height`)) true))