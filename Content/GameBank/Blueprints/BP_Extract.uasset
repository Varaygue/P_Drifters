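; BP_Extract is an extraction point where the player ends an exploration run.
; When the third-person character overlaps its Box, it passes the character's inventory items to the game instance, resets several run flags and triggers the exploration summary.
; It then calls Extract on the character, registers itself as the current extract and fades the player HUD through W_PlayerHUD.
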(event `self.Box.OnComponentBeginOverlap`
  (params (OverlappedComponent :type "PrimitiveComponent Object Reference") (OtherActor :type "Actor Object Reference") (OtherComp :type "PrimitiveComponent Object Reference") (OtherBodyIndex :type Integer) (bFromSweep :type Boolean) (SweepResult :type "HitResult Structure (by ref)"))
  (bind _asgi_game_instance (cast `/Game/GameBank/Blueprints/GameInstance/GI_GameInstance` (`GameplayStatics.GetGameInstance`) :!pure true))
  (bind _asbp_third_person_character (cast `/Game/GameBank/Blueprints/Characters/Player/Zone/BP_ThirdPersonCharacter` OtherActor))
  (`/Game/GameBank/Blueprints/GameInstance/GI_GameInstance.TransferInventory` _asgi_game_instance (`/Game/GameBank/Blueprints/Ingredients/Inventory/BP_InventoryComponent.Items` (`/Game/GameBank/Blueprints/Characters/Player/Zone/BP_ThirdPersonCharacter.BP_InventoryComponent` _asbp_third_person_character)))
  (set `/Game/GameBank/Blueprints/GameInstance/GI_GameInstance.FirstInventoryOpen` false _asgi_game_instance)
  (`/Game/GameBank/Blueprints/GameInstance/GI_GameInstance.ExplorationSummary` _asgi_game_instance)
  (set `/Game/GameBank/Blueprints/GameInstance/GI_GameInstance.DaySpent` false _asgi_game_instance)
  (`/Game/GameBank/Blueprints/Characters/Player/Zone/BP_ThirdPersonCharacter.Extract` _asbp_third_person_character)
  (set `/Game/GameBank/Blueprints/GameInstance/GI_GameInstance.LeavingCamp` false _asgi_game_instance)
  (set `/Game/GameBank/Blueprints/Characters/Player/Zone/BP_ThirdPersonCharacter.CurrentExtract` self _asbp_third_person_character)
  (bind _foundwidgets (`WidgetBlueprintLibrary.GetAllWidgetsOfClass` "/Game/GameBank/Blueprints/Widgets/W_PlayerHUD.W_PlayerHUD_C"))
  (`/Game/GameBank/Blueprints/Widgets/W_PlayerHUD.ExtractHUDFade` (`|GetArrayItem` _foundwidgets)))

(fn `UserConstructionScript`)