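; Game instance that persists camp resources, progression flags and gathered loot for a camp and exploration game.
; TransferInventory adds unique item references to a cached inventory, then totals their values by type into cached food, health, hope, protection and tech.
; It also copies current resource values from the camp player and resets run state to defaults.
; EndGame and SetZoneExplored are empty stubs, and clearing cached resources leaves tech untouched.
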(fn `ClearCachedRessources`
  (set `self.CachedFood` 0.0)
  (set `self.CachedHealth` 0.0)
  (set `self.CachedHope` 0.0)
  (set `self.CachedProtection` 0.0))

(fn `EndGame`)

(fn `ExplorationSummary`
  (set `self.CanSummary` true))

(fn `GetValuesOfGatheredItems`
  (returns (TotalFood :type "Float (double-precision)") (TotalHealth :type "Float (double-precision)") (TotalHope :type "Float (double-precision)") (TotalProtection :type "Float (double-precision)") (TotalTech :type "Float (double-precision)"))
  (locals (`TotalFood (local)` :type "Float (double-precision)") (`TotalHealth (local)` :type "Float (double-precision)") (`TotalHope (local)` :type "Float (double-precision)") (`TotalProtection (local)` :type "Float (double-precision)") (`TotalTech (local)` :type "Float (double-precision)"))
  (for _array_element (`self.CachedInventory`)
    (`/Engine/EditorBlueprintResources/StandardMacros.IsValid` _array_element
      (:`Is Valid`
        (switch `/Game/GameBank/Blueprints/Ingredients/Inventory/E_ItemTypes` (`/Game/GameBank/Blueprints/Ingredients/Inventory/BP_BaseObject.Get Item Type` _array_element)
          (:`NewEnumerator3`
            (bind _value (`/Game/GameBank/Blueprints/Ingredients/Inventory/BP_BaseObject.Get Item Value` _array_element))
            (set `local.TotalFood (local)` (+ (`local.TotalFood (local)`) _value)))
          (:`NewEnumerator0`
            (set `local.TotalHealth (local)` (+ _value (`local.TotalHealth (local)`))))
          (:`NewEnumerator1`
            (bind _value_2 (`/Game/GameBank/Blueprints/Ingredients/Inventory/BP_BaseObject.Get Item Value` _array_element))
            (set `local.TotalHope (local)` (+ (`local.TotalHope (local)`) _value_2)))
          (:`NewEnumerator2`
            (set `local.TotalProtection (local)` (+ _value_2 (`local.TotalProtection (local)`))))
          (:`NewEnumerator5`
            (set `local.TotalTech (local)` (+ _value_2 (`local.TotalTech (local)`))))))))
  (return (`local.TotalFood (local)`) (`local.TotalHealth (local)`) (`local.TotalHope (local)`) (`local.TotalProtection (local)`) (`local.TotalTech (local)`)))

(fn `ResetGameInstance`
  (set `self.FoodValue` 60.0)
  (set `self.HealthValue` 60.0)
  (set `self.HopeValue` 60.0)
  (set `self.ProtectionValue` 30.0)
  (set `self.TechValue` 1.0)
  (set `self.CrisisOngoing` false)
  (set `self.CanteenBuilt` false)
  (set `self.ClinicBuilt` false)
  (set `self.CultBuilt` false)
  (set `self.WatchtowerBuilt` false)
  (set `self.DayCount` 5)
  (set `self.DaySpent` false)
  (set `self.LeavingCamp` false)
  (set `self.FirstTimeInCamp` true)
  (set `self.FirstInventoryOpen` true)
  (`self.ClearCachedRessources`)
  (`KismetArrayLibrary.Array_Clear` (`self.CompletedEventList`))
  (set `self.LastLevelPlayedData` (struct))
  (set `self.BuildingTutorial` false)
  (set `self.ObjectiveShown` false))

(fn `SetZoneExplored`)

(fn `TransferInventory`
  (params (PlayerInventory :type "Array of /Game/GameBank/Blueprints/Ingredients/Inventory/BP_BaseObject Object Reference"))
  ;[1 1 1] Get Only one reference to each item in Player Inventory
  (for _array_element PlayerInventory
    (`KismetArrayLibrary.Array_AddUnique` (`self.CachedInventory`) _array_element))
  (bind (_totalfood _totalhealth _totalhope _totalprotection _totaltech) (`self.GetValuesOfGatheredItems`))
  (set `self.CachedFood` _totalfood)
  (set `self.CachedHealth` _totalhealth)
  (set `self.CachedHope` _totalhope)
  (set `self.CachedProtection` _totalprotection)
  (set `self.CachedTech` _totaltech))

(fn `Update Camp Cached Ressources`
  (bind _asbp_player_camp (cast `/Game/GameBank/Blueprints/Characters/Player/Camp/BP_PlayerCamp` (`GameplayStatics.GetPlayerCharacter` 0) :!pure true))
  (set `self.FoodValue` (`/Game/GameBank/Blueprints/Characters/Player/Camp/BP_PlayerCamp.FoodCurrent` _asbp_player_camp))
  (set `self.HealthValue` (`/Game/GameBank/Blueprints/Characters/Player/Camp/BP_PlayerCamp.HealthCurrent` _asbp_player_camp))
  (set `self.HopeValue` (`/Game/GameBank/Blueprints/Characters/Player/Camp/BP_PlayerCamp.HopeCurrent` _asbp_player_camp))
  (set `self.ProtectionValue` (`/Game/GameBank/Blueprints/Characters/Player/Camp/BP_PlayerCamp.ProtCurrent` _asbp_player_camp))
  (set `self.TechValue` (`/Game/GameBank/Blueprints/Characters/Player/Camp/BP_PlayerCamp.TechCurrent` _asbp_player_camp)))