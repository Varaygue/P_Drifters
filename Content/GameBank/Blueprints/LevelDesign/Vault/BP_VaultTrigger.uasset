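; Vault trigger actor for the level that shows and hides a widget component on demand.
; Each ToggleWidget call alternates through a FlipFlop between showing and hiding the widget.
; On show, it pitches the widget toward the player camera once, with yaw fixed at 180 and no roll.
; The file contains no overlap or tick logic, only this toggle event.
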(event `self.ReceiveTick`
  (params (DeltaSeconds :type "Float (single-precision)")))

(event `ToggleWidget`
  (bind _widget (`self.Widget`))
  (`/Engine/EditorBlueprintResources/StandardMacros.FlipFlop`
    (:`A`
      (`SceneComponent.SetVisibility` _widget true false)
      (`SceneComponent.K2_SetWorldRotation` _widget (`KismetMathLibrary.MakeRotator` 0.0 (.pitch (`KismetMathLibrary.FindLookAtRotation` (`SceneComponent.K2_GetComponentLocation` (`self.Widget`)) (`PlayerCameraManager.GetCameraLocation` (`GameplayStatics.GetPlayerCameraManager` 0)))) 180.0) false false))
    (:`B`
      (`SceneComponent.SetVisibility` _widget false false))))

(fn `UserConstructionScript`)