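; Event system component that draws random narrative events and applies the resource outcome of the player's A/B choice.
; GetRandomEvent picks a DT_EventList row from EventRemaining, retries if it is in the GameInstance's CompletedEventList, otherwise records and returns it.
; Its removal re-rolls the random index, so the removed entry can differ from the drawn one.
; ResolveEvent adjusts BP_PlayerCamp resources, multiplying gains and applying losses without modifiers.
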(event `self.ReceiveBeginPlay`)

(fn `GetRandomEvent`
  (returns (`Out Row` :type "/Game/GameBank/Blueprints/Ingredients/EventSystem/S_EventInfo Structure") (Multiplier :type "Float (double-precision)"))
  (locals (`GameInstance (local)` :type "/Game/GameBank/Blueprints/GameInstance/GI_GameInstance Object Reference") (`Multiplier (local)` :type "Float (double-precision)" :default 1.0))
  (bind _eventremaining (`self.EventRemaining`))
  (bind _returnvalue (`KismetMathLibrary.RandomInteger` (- (`KismetArrayLibrary.Array_Length` _eventremaining) 1)))
  (set `local.GameInstance (local)` (cast `/Game/GameBank/Blueprints/GameInstance/GI_GameInstance` (`GameplayStatics.GetGameInstance`) :!pure true))
  (bind _returnvalue_2 (`|GetDataTableRow` "/Game/GameBank/Blueprints/Ingredients/EventSystem/DT_EventList.DT_EventList" (`|GetArrayItem` _eventremaining _returnvalue) :!label _label)
    (:`then`
      (`KismetArrayLibrary.Array_Remove` (`self.EventRemaining`) _returnvalue)
      (for _array_element (`/Game/GameBank/Blueprints/GameInstance/GI_GameInstance.CompletedEventList` (`local.GameInstance (local)`))
        (if (== (`.EventName_2_A824E65B4A80E7121823C4825B11B984` (break `/Game/GameBank/Blueprints/Ingredients/EventSystem/S_EventInfo` _array_element)) (`.EventName_2_A824E65B4A80E7121823C4825B11B984` (break `/Game/GameBank/Blueprints/Ingredients/EventSystem/S_EventInfo` _returnvalue_2)))
          (goto _label)))
      (`KismetArrayLibrary.Array_Add` (`/Game/GameBank/Blueprints/GameInstance/GI_GameInstance.CompletedEventList` (`local.GameInstance (local)`)) _returnvalue_2)
      (return _returnvalue_2 0.0))))

(fn `ResolveEvent`
  (params (`Is ChoiceA` :type Boolean) (Event :type "/Game/GameBank/Blueprints/Ingredients/EventSystem/S_EventInfo Structure") (Multiplier :type "Float (double-precision)" :default 1.0))
  (bind (_eventname _eventdescription _eventimage _choiceatext _choiceagain _choicealose _choicebtext _choicebgain _choiceblose) (break `/Game/GameBank/Blueprints/Ingredients/EventSystem/S_EventInfo` Event))
  (bind _asbp_player_camp (cast `/Game/GameBank/Blueprints/Characters/Player/Camp/BP_PlayerCamp` (`GameplayStatics.GetPlayerCharacter` 0) :!pure true))
  (bind _asbp_player_camp_2 (cast `/Game/GameBank/Blueprints/Characters/Player/Camp/BP_PlayerCamp` (`GameplayStatics.GetPlayerCharacter` 0) :!pure true))
  (if `Is ChoiceA`
    ;[1 1 1] Resolve event with choice A
    (`/Game/GameBank/Blueprints/Characters/Player/Camp/BP_PlayerCamp.IncreaseResources` _asbp_player_camp_2 _choiceagain 0.0 Multiplier)
    (`/Game/GameBank/Blueprints/Characters/Player/Camp/BP_PlayerCamp.DecreaseResources` _asbp_player_camp_2 _choicealose false)
    (else
      ;[1 1 1] Resolve Event with choice B
      (`/Game/GameBank/Blueprints/Characters/Player/Camp/BP_PlayerCamp.IncreaseResources` _asbp_player_camp _choicebgain 0.0 Multiplier)
      (`/Game/GameBank/Blueprints/Characters/Player/Camp/BP_PlayerCamp.DecreaseResources` _asbp_player_camp _choiceblose false))))