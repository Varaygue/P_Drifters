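; Clickable building slot in the camp that toggles a building window.
; Hovering the cube shows or hides a fake outline mesh, and clicks alternate through a FlipFlop between creating the window and removing it while clearing the player's FocusedBuilding.
; BeginPlay caches the camp player and game instance, then after a short delay finds the camp interface and tutorial widgets.
; First-time tutorial logic is present but disconnected.
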(event `self.ReceiveBeginPlay`
  (bind _asbp_player_camp (cast `/Game/GameBank/Blueprints/Characters/Player/Camp/BP_PlayerCamp` (`GameplayStatics.GetPlayerCharacter` 0)))
  (set `self.PlayerWidget` _asbp_player_camp)
  (bind _asgi_game_instance (cast `/Game/GameBank/Blueprints/GameInstance/GI_GameInstance` (`GameplayStatics.GetGameInstance`)))
  (set `self.GameInstance` _asgi_game_instance)
  (`KismetSystemLibrary.Delay` 0.5)
  (bind _foundwidgets (`WidgetBlueprintLibrary.GetAllWidgetsOfClass` "/Game/GameBank/HUD/Widgets/Player/Camp/WBP_CampInterface.WBP_CampInterface_C"))
  (set `self.W_Campinterface` (`|GetArrayItem` _foundwidgets))
  (bind _foundwidgets_2 (`WidgetBlueprintLibrary.GetAllWidgetsOfClass` "/Game/GameBank/HUD/Widgets/Player/Camp/Tutorial/WBP_CampTutorial01.WBP_CampTutorial01_C"))
  (set `self.CampTutorial` (`|GetArrayItem` _foundwidgets_2)))

(event `self.Cube.OnBeginCursorOver`
  (params (TouchedComponent :type "PrimitiveComponent Object Reference"))
  (`SceneComponent.SetVisibility` (`self.FakeOutline`) true false))

(event `self.Cube.OnEndCursorOver`
  (params (TouchedComponent :type "PrimitiveComponent Object Reference"))
  (`SceneComponent.SetVisibility` (`self.FakeOutline`) false false))

(event `self.Cube.OnClicked`
  (params (TouchedComponent :type "PrimitiveComponent Object Reference") (ButtonPressed :type "Key Structure"))
  (`/Engine/EditorBlueprintResources/StandardMacros.FlipFlop`
    (:`A`
      (bind _returnvalue (`|CreateWidget` "/Game/GameBank/HUD/Widgets/Player/Camp/BuildingWindows/WBP_BuildingWindow.WBP_BuildingWindow_C"))
      (bind _output_get (set `self.BuildWidget` _returnvalue))
      (`UserWidget.AddToViewport` _output_get 0))
    (:`B`
      (`Widget.RemoveFromParent` (`self.BuildWidget`))
      (set `/Game/GameBank/Blueprints/Characters/Player/Camp/BP_PlayerCamp.FocusedBuilding` null (`self.PlayerWidget`)))))

(fn `UserConstructionScript`)