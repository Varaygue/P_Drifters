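; Clickable camp building actor for the canteen, clinic, cult and watchtower types, with a widget icon.
; On BeginPlay it reads its built flag from the game instance by BuildingType and shows the matching level mesh, Niveau1 or Niveau2.
; Clicking the box or icon advances the first-time tutorial and, if clickable, moves the player camera to the building and opens a window with its name and description.
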(event `self.ReceiveBeginPlay`
  (bind _asbp_player_camp (cast `/Game/GameBank/Blueprints/Characters/Player/Camp/BP_PlayerCamp` (`GameplayStatics.GetPlayerCharacter` 0)))
  (set `self.PlayerReference` _asbp_player_camp)
  (bind _output_get (set `self.Status` (`self.GetGameInstanceBuilt` (cast `/Game/GameBank/Blueprints/GameInstance/GI_GameInstance` (`GameplayStatics.GetGameInstance`) :!pure true))))
  (`self.SetBuildingMeshState` _output_get)
  (bind _asbuilding_icons (cast `/Game/GameBank/HUD/Widgets/Player/Camp/BuildingWindows/BuildingIcons` (`WidgetComponent.GetWidget` (`self.BuildingIcon`))))
  (set `/Game/GameBank/HUD/Widgets/Player/Camp/BuildingWindows/BuildingIcons.IconTexture` (`self.BuildingIconTexture`) _asbuilding_icons))

(event `self.Box.OnClicked`
  (params (TouchedComponent :type "PrimitiveComponent Object Reference") (ButtonPressed :type "Key Structure"))
  (bind _playerreference (`self.PlayerReference`))
  (bind _activewindowbuilding (`self.ActiveWindowBuilding`))
  (bind _asgi_game_instance (cast `/Game/GameBank/Blueprints/GameInstance/GI_GameInstance` (`GameplayStatics.GetGameInstance`) :!label _label))
  (if (`/Game/GameBank/Blueprints/GameInstance/GI_GameInstance.FirstTimeInCamp` _asgi_game_instance)
    (`/Game/GameBank/HUD/Widgets/Player/Camp/Tutorial/WBP_CampTutorial.NextText` (`/Game/GameBank/Blueprints/Characters/Player/Camp/BP_PlayerCamp.CampTutorial` (`self.PlayerReference`))))
  (if (`self.bisClickable`)
    (set `/Game/GameBank/Blueprints/Characters/Player/Camp/BP_PlayerCamp.FocusedBuilding` self _playerreference)
    (set `/Game/GameBank/Blueprints/Characters/Player/Camp/BP_PlayerCamp.SelectedCamera` (`self.AttachedCamera`) _playerreference)
    (`/Game/GameBank/Blueprints/Characters/Player/Camp/BP_PlayerCamp.CameraMovement` _playerreference)
    (bind _returnvalue (`|CreateWidget` "/Game/GameBank/HUD/Widgets/Player/Camp/BuildingWindows/WBP_BuildingWindow.WBP_BuildingWindow_C"))
    (bind _output_get (set `self.ActiveWindowBuilding` _returnvalue))
    (`UserWidget.AddToViewport` _output_get 0)
    (`|ExecutionSequence`
      (:`then_0`
        (set `TextBlock.Text` (`self.Name`) (`/Game/GameBank/HUD/Widgets/Player/Camp/BuildingWindows/WBP_BuildingWindow.BuildingName` _activewindowbuilding)))
      (:`then_1`
        (set `TextBlock.Text` (`self.EffetDesc`) (`/Game/GameBank/HUD/Widgets/Player/Camp/BuildingWindows/WBP_BuildingWindow.BuildingDesc` _activewindowbuilding))))))

(event `self.BuildingIcon.OnClicked`
  (params (TouchedComponent :type "PrimitiveComponent Object Reference") (ButtonPressed :type "Key Structure"))
  (goto _label))

(fn `CallClick`)

(fn `GetGameInstanceBuilt`
  (params (`Game Instance` :type "/Game/GameBank/Blueprints/GameInstance/GI_GameInstance Object Reference"))
  (returns (IsBuilt :type Boolean))
  (switch `/Game/GameBank/Blueprints/Ingredients/Camp/Building/E_BuildingTypes` (`self.BuildingType`)
    (:`NewEnumerator0`
      (return (`/Game/GameBank/Blueprints/GameInstance/GI_GameInstance.CanteenBuilt` (`local.Game Instance`))))
    (:`NewEnumerator1`
      (return (`/Game/GameBank/Blueprints/GameInstance/GI_GameInstance.ClinicBuilt` (`local.Game Instance`))))
    (:`NewEnumerator2`
      (return (`/Game/GameBank/Blueprints/GameInstance/GI_GameInstance.CultBuilt` (`local.Game Instance`))))
    (:`NewEnumerator3`
      (return (`/Game/GameBank/Blueprints/GameInstance/GI_GameInstance.WatchtowerBuilt` (`local.Game Instance`))))))

(fn `SetBuildingMeshState`
  (params (Upgraded :type Boolean))
  (if Upgraded
    (`SceneComponent.SetVisibility` (`StaticMeshActor.StaticMeshComponent` (`self.Niveau1`)) false false)
    (`SceneComponent.SetVisibility` (`StaticMeshActor.StaticMeshComponent` (`self.Niveau2`)) true false)
    (else
      (`SceneComponent.SetVisibility` (`StaticMeshActor.StaticMeshComponent` (`self.Niveau1`)) true false)
      (`SceneComponent.SetVisibility` (`StaticMeshActor.StaticMeshComponent` (`self.Niveau2`)) false false))))

(fn `SetGameInstanceBuilt`
  (params (GameInstance :type "/Game/GameBank/Blueprints/GameInstance/GI_GameInstance Object Reference") (Value :type Boolean))
  (switch `/Game/GameBank/Blueprints/Ingredients/Camp/Building/E_BuildingTypes` (`self.BuildingType`)
    (:`NewEnumerator0`
      (set `/Game/GameBank/Blueprints/GameInstance/GI_GameInstance.CanteenBuilt` (`local.Value`) (`local.GameInstance`)))
    (:`NewEnumerator1`
      (set `/Game/GameBank/Blueprints/GameInstance/GI_GameInstance.ClinicBuilt` (`local.Value`) (`local.GameInstance`)))
    (:`NewEnumerator2`
      (set `/Game/GameBank/Blueprints/GameInstance/GI_GameInstance.CultBuilt` (`local.Value`) (`local.GameInstance`)))
    (:`NewEnumerator3`
      (set `/Game/GameBank/Blueprints/GameInstance/GI_GameInstance.WatchtowerBuilt` (`local.Value`) (`local.GameInstance`)))))

(fn `UserConstructionScript`)