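; BP_VaultTutorial6 is a one-shot tutorial trigger that spawns an enemy when the player enters its box.
; The first overlap by BP_ThirdPersonCharacter spawns a BP_Enemy offset along world X from the ToDestroy actor, rotated along that actor's direction to the player.
; ToDestroy is then moved 1500 units upward instead of being destroyed, despite its name.
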(event `self.Box.OnComponentBeginOverlap`
  (params (OverlappedComponent :type "PrimitiveComponent Object Reference") (OtherActor :type "Actor Object Reference") (OtherComp :type "PrimitiveComponent Object Reference") (OtherBodyIndex :type Integer) (bFromSweep :type Boolean) (SweepResult :type "HitResult Structure (by ref)"))
  (bind _todestroy (`self.ToDestroy`))
  (bind _returnvalue (`self.K2_GetActorLocation` _todestroy))
  (bind _asbp_third_person_character (cast `/Game/GameBank/Blueprints/Characters/Player/Zone/BP_ThirdPersonCharacter` OtherActor))
  (`/Engine/EditorBlueprintResources/StandardMacros.DoOnce` false
    (:`Completed`
      (`|SpawnActorFromClass` :`Class` "/Game/GameBank/Blueprints/Characters/AI/BP_Enemy.BP_Enemy_C" :`SpawnTransform` (`KismetMathLibrary.MakeTransform` (+ _returnvalue (-350.0 0.0 0.0)) (`KismetMathLibrary.FindLookAtRotation` (`self.K2_GetActorLocation` _todestroy) (`self.K2_GetActorLocation` _asbp_third_person_character))) :`CollisionHandlingOverride` "AdjustIfPossibleButAlwaysSpawn" :`TransformScaleMethod` "MultiplyWithRoot" :`Instigator` null)
      (`self.K2_SetActorLocation` _todestroy (- _returnvalue (0.0 0.0 -1500.0)) false false))))

(fn `UserConstructionScript`)