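; Tutorial trigger volume that sends the player back to a set location with a monster warning while the tutorial enemy exists.
; On box overlap, it disables the character's input, shows WBP_MonsterWarning and moves the character to the TeleportLocation actor.
; It finds BP_EnemyTutorial at BeginPlay and checks it every Tick, destroying itself once that enemy is no longer valid.
; Input is not re-enabled in this Blueprint.
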(event `self.ReceiveBeginPlay`
  (bind _returnvalue (`GameplayStatics.GetActorOfClass` "/Game/GameBank/Blueprints/Characters/AI/BP_EnemyTutorial.BP_EnemyTutorial_C"))
  (set `self.EnemyReference` _returnvalue))

(event `self.ReceiveTick`
  (params (DeltaSeconds :type "Float (single-precision)"))
  (`self.EnemyReference`
    (:`then`)
    (:`else`
      (`self.K2_DestroyActor`))))

(event `self.Box.OnComponentBeginOverlap`
  (params (OverlappedComponent :type "PrimitiveComponent Object Reference") (OtherActor :type "Actor Object Reference") (OtherComp :type "PrimitiveComponent Object Reference") (OtherBodyIndex :type Integer) (bFromSweep :type Boolean) (SweepResult :type "HitResult Structure (by ref)"))
  (bind _asbp_third_person_character (cast `/Game/GameBank/Blueprints/Characters/Player/Zone/BP_ThirdPersonCharacter` OtherActor))
  (bind _output_get (set `self.PlayerReference` _asbp_third_person_character))
  (`self.DisableInput` _output_get (`GameplayStatics.GetPlayerController` 0))
  (bind _returnvalue (`|CreateWidget` "/Game/GameBank/Blueprints/Ingredients/TutorialTriggers/TPBack/WBP_MonsterWarning.WBP_MonsterWarning_C"))
  (bind _output_get_2 (set `self.WarningWidget` _returnvalue))
  (`UserWidget.AddToViewport` _output_get_2 0)
  (`self.K2_SetActorLocation` (`self.PlayerReference`) (`self.K2_GetActorLocation` (`self.TeleportLocation`)) false false))

(fn `UserConstructionScript`)