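; BP_BaseItem is a base actor for world items that can be picked up into an inventory.
; On BeginPlay it fills an unset ItemObject from GetDefaultItemObject, which returns nothing here and appears intended for child Blueprints to override.
; InteractItem passes that object to the given InventoryComponent's TryAddItem.
; On success it plays the 2D ItemPickup audio event and destroys the actor, otherwise it prints a failure message.
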(event `self.ReceiveBeginPlay`
  (`/Engine/EditorBlueprintResources/StandardMacros.IsValid` (`self.ItemObject`)
    (:`Is Not Valid`
      (bind _itemobject (`self.Get Default Item Object`))
      (set `self.ItemObject` _itemobject))))

(event `/Game/GameBank/Blueprints/Ingredients/Inventory/BPI_InteractItem.InteractItem`
  (params (InventoryComponent :type "/Game/GameBank/Blueprints/Ingredients/Inventory/BP_InventoryComponent Object Reference") (InventoryWidget :type "/Game/GameBank/Blueprints/Widgets/Inventory/W_InventorySpatial Object Reference"))
  (bind _added (`/Game/GameBank/Blueprints/Ingredients/Inventory/BP_InventoryComponent.TryAddItem` InventoryComponent (`self.ItemObject`)))
  (if _added
    (`FMODBlueprintStatics.PlayEvent2D` "/Game/FMOD/Events/Inventory/ItemPickup.ItemPickup")
    (`self.K2_DestroyActor`)
    (else
      (`KismetSystemLibrary.PrintString` "Failed to add item"))))

(fn `Get Default Item Object`
  (returns (ItemObject :type "/Game/GameBank/Blueprints/Ingredients/Inventory/BP_BaseObject Object Reference"))
  (return null))

(fn `UserConstructionScript`)