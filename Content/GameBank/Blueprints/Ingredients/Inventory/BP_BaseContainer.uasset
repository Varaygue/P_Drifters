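; Base lootable container actor with a grid inventory, optionally locked behind a key item.
; On BeginPlay it sizes the grid and fills it from DT_Items, using its item list as given or picked randomly.
; Interaction consumes a key if locked, then opens the container UI, changes mesh stencils and may show a tutorial, or shows a locked popup.
; When non-empty, overlap plus a line-of-sight trace reveals a camera-pitched prompt widget.
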(event `self.ReceiveBeginPlay`
  (`self.InitializeSize`)
  (`self.BuildInventory` (`self.ItemList`) (`self.ShouldRandomize`)))

(event `/Game/GameBank/Blueprints/Ingredients/Inventory/BPI_InteractItem.InteractItem`
  (params (InventoryComponent :type "/Game/GameBank/Blueprints/Ingredients/Inventory/BP_InventoryComponent Object Reference") (InventoryWidget :type "/Game/GameBank/Blueprints/Widgets/Inventory/W_InventorySpatial Object Reference") (Initiator :type "/Game/GameBank/Blueprints/Characters/Player/Zone/BP_ThirdPersonCharacter Object Reference"))
  (bind _allitems (`/Game/GameBank/Blueprints/Ingredients/Inventory/BP_InventoryComponent.GetAllItems` InventoryComponent))
  (bind _keys (`BlueprintMapLibrary.Map_Keys` _allitems))
  (for _array_element _keys
    (if (and (`/Game/GameBank/Blueprints/Ingredients/Inventory/BP_BaseObject.Get IsKey` _array_element) (`self.IsLocked`))
      (`/Game/GameBank/Blueprints/Ingredients/Inventory/BP_InventoryComponent.RemoveItem` InventoryComponent _array_element)
      (set `self.IsLocked` false)
      (break)))
  (if (`self.IsLocked`)
    (bind _returnvalue (`|CreateWidget` "/Game/GameBank/Blueprints/Widgets/W_InventoryFull.W_InventoryFull_C"))
    (set `TextBlock.Text` "C'est fermé, il faut trouver une clé ..." (`/Game/GameBank/Blueprints/Widgets/W_InventoryFull.Text_Popup` _returnvalue))
    (`UserWidget.AddToViewport` _returnvalue 0)
    (else
      (`/Game/GameBank/Blueprints/Widgets/Inventory/W_InventoryGrid.Initialize` (`/Game/GameBank/Blueprints/Widgets/Inventory/W_InventorySpatial.W_InventoryGrid_Container` InventoryWidget) (`self.BP_InventoryComponent`) (`/Game/GameBank/Blueprints/Widgets/Inventory/W_InventorySpatial.TileSize` InventoryWidget))
      (`/Game/GameBank/Blueprints/Widgets/Inventory/W_InventorySpatial.ShowContainer` InventoryWidget)
      (`/Game/GameBank/Blueprints/Characters/Player/Zone/BP_ThirdPersonCharacter.ShowInventory` Initiator)
      (for _array_element_2 (`self.MeshRefs`)
        (`PrimitiveComponent.SetCustomDepthStencilValue` (`StaticMeshActor.StaticMeshComponent` _array_element_2) 2)
        (bind _asgi_game_instance (cast `/Game/GameBank/Blueprints/GameInstance/GI_GameInstance` (`GameplayStatics.GetGameInstance`)))
        (if (`/Game/GameBank/Blueprints/GameInstance/GI_GameInstance.FirstInventoryOpen` _asgi_game_instance)
          (if (`/Game/GameBank/Blueprints/GameInstance/GI_GameInstance.FirstTimeInCamp` _asgi_game_instance)
            (bind _returnvalue_2 (`|CreateWidget` "/Game/GameBank/Blueprints/Widgets/W_InputTutorial04.W_InputTutorial04_C"))
            (`UserWidget.AddToViewport` _returnvalue_2 0)))))))

(event `self.ReceiveActorBeginOverlap`
  (params (OtherActor :type "Actor Object Reference"))
  (bind _widget (`self.Widget`))
  (bind _outhit (`KismetSystemLibrary.LineTraceSingle` :`Start` (`self.K2_GetActorLocation` OtherActor) :`End` (`self.GetActorBounds` true true) :`TraceChannel` "TraceTypeQuery1" :`bIgnoreSelf` false))
  (bind _allitems (`/Game/GameBank/Blueprints/Ingredients/Inventory/BP_InventoryComponent.GetAllItems` (`self.BP_InventoryComponent`)))
  (if (and (> (`BlueprintMapLibrary.Map_Length` _allitems) 0) (== (`GameplayStatics.GetObjectClass` OtherActor) "/Game/GameBank/Blueprints/Characters/Player/Zone/BP_ThirdPersonCharacter.BP_ThirdPersonCharacter_C") (== (`.HitActor` (`GameplayStatics.BreakHitResult` _outhit)) self))
    (`SceneComponent.SetVisibility` _widget true false)
    (`SceneComponent.K2_SetWorldRotation` _widget (`KismetMathLibrary.MakeRotator` 0.0 (.pitch (`KismetMathLibrary.FindLookAtRotation` (`SceneComponent.K2_GetComponentLocation` (`self.Widget`)) (`PlayerCameraManager.GetCameraLocation` (`GameplayStatics.GetPlayerCameraManager` 0)))) 180.0) false false)))

(event `self.ReceiveActorEndOverlap`
  (params (OtherActor :type "Actor Object Reference"))
  (`SceneComponent.SetVisibility` (`self.Widget`) false false))

(fn `BuildInventory`
  (params (NameList :type "Array of Name") (ShouldRandomize :type Boolean))
  (bind _numbervariance (`self.NumberVariance`))
  (if ShouldRandomize
    (for _ (range 1 (+ (+ (`self.NumberOfItems`) (`KismetMathLibrary.RandomIntegerInRange` (* _numbervariance -1) _numbervariance)) 1))
      (bind _returnvalue (`|GetDataTableRow` "/Game/GameBank/Blueprints/Ingredients/Inventory/DT_Items.DT_Items" (`KismetArrayLibrary.Array_Random` (`local.NameList`)))
        (:`then`
          (bind _returnvalue_2 (`|GenericCreateObject` "/Game/GameBank/Blueprints/Ingredients/Inventory/BP_BaseObject.BP_BaseObject_C" (make `IntPoint` (`.ItemSizeX_34_7675B9184F4232D46117A39966428D8A` (break `/Game/GameBank/Blueprints/Ingredients/Inventory/S_ItemInfo` _returnvalue)) (`.ItemSizeY_35_5C86D98F4F688FC3BFD2EFAD9AE2EF15` (break `/Game/GameBank/Blueprints/Ingredients/Inventory/S_ItemInfo` _returnvalue))) (`.ItemName_40_AD9C8E734D28ECDCC012BDA7BC249166` (break `/Game/GameBank/Blueprints/Ingredients/Inventory/S_ItemInfo` _returnvalue)) (break `/Game/GameBank/Blueprints/Ingredients/Inventory/S_ItemInfo` _returnvalue) (`.Value_49_4341E4074924F624F8D693B25295D0AC` (break `/Game/GameBank/Blueprints/Ingredients/Inventory/S_ItemInfo` _returnvalue)) (`.Icon_55_2515C8234B008FF94BA3CE9B57BA8192` (break `/Game/GameBank/Blueprints/Ingredients/Inventory/S_ItemInfo` _returnvalue)) (`.IconRotated_56_F690AA7C437BE1FD017B9F9C7E6FB131` (break `/Game/GameBank/Blueprints/Ingredients/Inventory/S_ItemInfo` _returnvalue)) (`.ItemClass_44_D9764F3344DCDF850AA3128BA6D074C4` (break `/Game/GameBank/Blueprints/Ingredients/Inventory/S_ItemInfo` _returnvalue)) (`.IsKey_50_FC2CEEC7487E35345C82769430C3AD5D` (break `/Game/GameBank/Blueprints/Ingredients/Inventory/S_ItemInfo` _returnvalue)) (`.ItemEffect_48_3C70D77F4CA2A42423D762962E481CF6` (break `/Game/GameBank/Blueprints/Ingredients/Inventory/S_ItemInfo` _returnvalue)) 0 null))
          (`/Game/GameBank/Blueprints/Ingredients/Inventory/BP_InventoryComponent.TryAddItem` (`self.BP_InventoryComponent`) _returnvalue_2))))
    (else
      (for _array_element NameList
        (bind _returnvalue_3 (`|GetDataTableRow` "/Game/GameBank/Blueprints/Ingredients/Inventory/DT_Items.DT_Items" _array_element)
          (:`then`
            (bind _returnvalue_4 (`|GenericCreateObject` "/Game/GameBank/Blueprints/Ingredients/Inventory/BP_BaseObject.BP_BaseObject_C" (make `IntPoint` (`.ItemSizeX_34_7675B9184F4232D46117A39966428D8A` (break `/Game/GameBank/Blueprints/Ingredients/Inventory/S_ItemInfo` _returnvalue_3)) (`.ItemSizeY_35_5C86D98F4F688FC3BFD2EFAD9AE2EF15` (break `/Game/GameBank/Blueprints/Ingredients/Inventory/S_ItemInfo` _returnvalue_3))) (`.ItemName_40_AD9C8E734D28ECDCC012BDA7BC249166` (break `/Game/GameBank/Blueprints/Ingredients/Inventory/S_ItemInfo` _returnvalue_3)) (break `/Game/GameBank/Blueprints/Ingredients/Inventory/S_ItemInfo` _returnvalue_3) (`.Value_49_4341E4074924F624F8D693B25295D0AC` (break `/Game/GameBank/Blueprints/Ingredients/Inventory/S_ItemInfo` _returnvalue_3)) (`.Icon_55_2515C8234B008FF94BA3CE9B57BA8192` (break `/Game/GameBank/Blueprints/Ingredients/Inventory/S_ItemInfo` _returnvalue_3)) (`.IconRotated_56_F690AA7C437BE1FD017B9F9C7E6FB131` (break `/Game/GameBank/Blueprints/Ingredients/Inventory/S_ItemInfo` _returnvalue_3)) (`.ItemClass_44_D9764F3344DCDF850AA3128BA6D074C4` (break `/Game/GameBank/Blueprints/Ingredients/Inventory/S_ItemInfo` _returnvalue_3)) (`.IsKey_50_FC2CEEC7487E35345C82769430C3AD5D` (break `/Game/GameBank/Blueprints/Ingredients/Inventory/S_ItemInfo` _returnvalue_3)) (`.ItemEffect_48_3C70D77F4CA2A42423D762962E481CF6` (break `/Game/GameBank/Blueprints/Ingredients/Inventory/S_ItemInfo` _returnvalue_3)) 0 null))
            (`/Game/GameBank/Blueprints/Ingredients/Inventory/BP_InventoryComponent.TryAddItem` (`self.BP_InventoryComponent`) _returnvalue_4)))))))

(fn `InitializeSize`
  (bind _bp_inventorycomponent (`self.BP_InventoryComponent`))
  (set `/Game/GameBank/Blueprints/Ingredients/Inventory/BP_InventoryComponent.Columns` (`self.ContainerSizeX`) _bp_inventorycomponent)
  (set `/Game/GameBank/Blueprints/Ingredients/Inventory/BP_InventoryComponent.Rows` (`self.ContainerSizeY`) _bp_inventorycomponent)
  (`/Game/GameBank/Blueprints/Ingredients/Inventory/BP_InventoryComponent.ResizeInventory` _bp_inventorycomponent))

(fn `UserConstructionScript`)