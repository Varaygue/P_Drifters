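; Base interactable actor for world items that the player can pick up.
; The construction script converts the ItemName enum to a row name and loads the matching DT_Items row into ItemInfo.
; InteractItem passes ItemInfo to PickupItem on the player's BP_ThirdPersonCharacter and destroys the actor only if that pickup succeeds.
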(event `/Game/GameBank/Blueprints/Ingredients/Inventory/BPI_InteractItem.InteractItem`
  (bind _asbp_third_person_character (cast `/Game/GameBank/Blueprints/Characters/Player/Zone/BP_ThirdPersonCharacter` (`GameplayStatics.GetPlayerCharacter` 0)))
  (bind _pickedup (`/Game/GameBank/Blueprints/Characters/Player/Zone/BP_ThirdPersonCharacter.PickupItem` _asbp_third_person_character (`self.ItemInfo`)))
  (if _pickedup
    (`self.K2_DestroyActor`)))

(fn `UserConstructionScript`
  (bind _returnvalue (`|GetDataTableRow` "/Game/GameBank/Blueprints/Ingredients/Inventory/DT_Items.DT_Items" (`KismetStringLibrary.Conv_StringToName` (`|GetEnumeratorNameAsString` (`self.ItemName`))))
    (:`then`
      (set `self.ItemInfo` _returnvalue))))