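; Base hiding spot actor, such as a closet, that lets the player hide inside and step back out.
; Overlap by the third-person character shows an interact prompt turned toward the camera, if a line trace confirms the spot is unobstructed.
; Interacting toggles hiding: mesh visibility, collision, movement and rotation switch, the player moves inside or out in front, and sounds play.
; Entering also turns off the flashlight and notifies the vault enemy tutorial if present.
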(event `self.ReceiveActorBeginOverlap`
  (params (OtherActor :type "Actor Object Reference"))
  (bind _interacttext (`self.InteractText`))
  (bind _outhit (`KismetSystemLibrary.LineTraceSingle` :`Start` (`self.K2_GetActorLocation` OtherActor) :`End` (`self.GetActorBounds` true true) :`TraceChannel` "TraceTypeQuery1" :`bIgnoreSelf` false))
  (if (and (== (`.HitActor` (`GameplayStatics.BreakHitResult` _outhit)) self) (== (`GameplayStatics.GetObjectClass` OtherActor) "/Game/GameBank/Blueprints/Characters/Player/Zone/BP_ThirdPersonCharacter.BP_ThirdPersonCharacter_C"))
    (`SceneComponent.SetVisibility` _interacttext true false)
    (`SceneComponent.K2_SetWorldRotation` _interacttext (`KismetMathLibrary.MakeRotator` 0.0 (.pitch (`KismetMathLibrary.FindLookAtRotation` (`SceneComponent.K2_GetComponentLocation` _interacttext) (`PlayerCameraManager.GetCameraLocation` (`GameplayStatics.GetPlayerCameraManager` 0)))) 180.0) false false)))

(event `self.ReceiveActorEndOverlap`
  (params (OtherActor :type "Actor Object Reference"))
  (`SceneComponent.SetVisibility` (`self.InteractText`) false false))

(event `/Game/GameBank/Blueprints/Ingredients/Inventory/BPI_InteractItem.InteractItem`
  (params (InventoryComponent :type "/Game/GameBank/Blueprints/Ingredients/Inventory/BP_InventoryComponent Object Reference") (InventoryWidget :type "/Game/GameBank/Blueprints/Widgets/Inventory/W_InventorySpatial Object Reference") (Initiator :type "/Game/GameBank/Blueprints/Characters/Player/Zone/BP_ThirdPersonCharacter Object Reference"))
  (bind (_returnvalue_x _returnvalue_y) (`KismetMathLibrary.BreakVector` (`self.K2_GetActorLocation`)))
  (bind _capsulecomponent (`Character.CapsuleComponent` Initiator))
  (bind _initiator (`self.Initiator`))
  (bind _initiator_2 (`self.Initiator`))
  (bind _initiator_3 (`self.Initiator`))
  (bind _mesh (`Character.Mesh` Initiator))
  (bind _returnvalue (`self.K2_GetActorLocation` _initiator_3))
  (bind _charactermovement (`Character.CharacterMovement` _initiator))
  (set `self.Initiator` Initiator)
  (if (`/Game/GameBank/Blueprints/Characters/Player/Zone/BP_ThirdPersonCharacter.isHiding` (`self.Initiator`))
    (`SceneComponent.SetVisibility` _mesh true false)
    (`PrimitiveComponent.SetCollisionEnabled` _capsulecomponent "QueryAndPhysics")
    (`self.K2_SetActorLocation` _initiator (+ _returnvalue (* (`self.GetActorForwardVector`) 100.0)) false false)
    (`CharacterMovementComponent.SetMovementMode` _charactermovement "MOVE_Walking" 0)
    (set `/Game/GameBank/Blueprints/Characters/Player/Zone/BP_ThirdPersonCharacter.isHiding` false _initiator_2)
    (set `/Game/GameBank/Blueprints/Characters/Player/Zone/BP_ThirdPersonCharacter.CanRotate` true _initiator_2)
    (`GameplayStatics.PlaySoundAtLocation` "/Game/GameBank/SFX/SoundEffects/Player/SFX_Player_Hide_Closet_Out.SFX_Player_Hide_Closet_Out" (`self.K2_GetActorLocation`) (struct) 1.0 1.0 0.0 null null null null)
    (set `self.IsPlayerInside` false)
    (else
      (`SceneComponent.SetVisibility` _mesh false false)
      (`PrimitiveComponent.SetCollisionEnabled` _capsulecomponent "NoCollision")
      (`self.K2_SetActorLocationAndRotation` _initiator (`KismetMathLibrary.MakeVector` _returnvalue_x _returnvalue_y (.z _returnvalue)) (`self.K2_GetActorRotation` _initiator_3) false false)
      (`CharacterMovementComponent.SetMovementMode` _charactermovement "MOVE_None" 0)
      (set `/Game/GameBank/Blueprints/Characters/Player/Zone/BP_ThirdPersonCharacter.isHiding` true _initiator_2)
      (set `/Game/GameBank/Blueprints/Characters/Player/Zone/BP_ThirdPersonCharacter.flashlightOn` false _initiator_2)
      (set `/Game/GameBank/Blueprints/Characters/Player/Zone/BP_ThirdPersonCharacter.CanRotate` false _initiator_2)
      (set `self.IsPlayerInside` true)
      (`GameplayStatics.PlaySoundAtLocation` "/Game/GameBank/SFX/SoundEffects/Player/SFX_Player_Hide_Closet_In.SFX_Player_Hide_Closet_In" (`self.K2_GetActorLocation`) (struct) 1.0 1.0 0.0 null null null null)
      (bind _returnvalue_2 (`GameplayStatics.GetActorOfClass` "/Game/GameBank/Blueprints/BP_VaultTutorial7.BP_VaultTutorial7_C"))
      (set `self.EnemyTutorial` _returnvalue_2)
      (bind _enemytutorial (`self.EnemyTutorial`)
        (:`then`
          (`/Game/GameBank/Blueprints/BP_VaultTutorial7.EnemyTutorial` _enemytutorial))
        (:`else`)))))

(fn `UserConstructionScript`)