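; Toxic plant hazard that drains the player's LifePoints while they stand inside its Cube trigger volume.
; On overlap it shows a toxic post-process and a hit widget, then repeatedly subtracts DamageRate through a short delay loop.
; Tick replays a cough sound, throttled by a DoOnce and Delay, while the player is inside.
; End overlap hides the effect, removes the widget and re-arms the trigger.
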(event `self.ReceiveTick`
  (params (DeltaSeconds :type "Float (single-precision)"))
  (if (`self.PlayerInside`)
    (`/Engine/EditorBlueprintResources/StandardMacros.DoOnce` false :!label _label
      (:`Completed`
        (`GameplayStatics.PlaySound2D` "/Game/GameBank/SFX/SoundEffects/Player/SFX_PlayerCough_Cue.SFX_PlayerCough_Cue" 1.0 1.0 0.0 null null)
        (`KismetSystemLibrary.Delay` 1.5)
        (goto _label :!via `Reset`)))))

(event `self.Cube.OnComponentBeginOverlap`
  (params (OverlappedComponent :type "PrimitiveComponent Object Reference") (OtherActor :type "Actor Object Reference") (OtherComp :type "PrimitiveComponent Object Reference") (OtherBodyIndex :type Integer) (bFromSweep :type Boolean) (SweepResult :type "HitResult Structure (by ref)"))
  (`/Engine/EditorBlueprintResources/StandardMacros.DoOnce` false :!label _label_2
    (:`Completed`
      (bind _asbp_third_person_character (cast `/Game/GameBank/Blueprints/Characters/Player/Zone/BP_ThirdPersonCharacter` OtherActor))
      (`SceneComponent.SetVisibility` (`self.PostProcessToxic`) true false)
      (bind _returnvalue (`|CreateWidget` "/Game/GameBank/HUD/Widgets/Player/Zone/Damage/WBP_Hit.WBP_Hit_C"))
      (bind _output_get (set `self.FeedbackWidget` _returnvalue))
      (`UserWidget.AddToViewport` _output_get -2)
      (set `self.PlayerRef` _asbp_third_person_character)
      (set `self.PlayerInside` true)
      (bind _playerref (`self.PlayerRef`)
        (:`then`
          (set `/Game/GameBank/Blueprints/Characters/Player/Zone/BP_ThirdPersonCharacter.LifePoints` (- (`/Game/GameBank/Blueprints/Characters/Player/Zone/BP_ThirdPersonCharacter.LifePoints` _asbp_third_person_character) (`self.DamageRate`)) _playerref :!label _label_3)
          (`KismetSystemLibrary.RetriggerableDelay` 0.1)
          (if (`self.PlayerInside`)
            (goto _label_3)))
        (:`else`)))))

(event `self.Cube.OnComponentEndOverlap`
  (params (OverlappedComponent :type "PrimitiveComponent Object Reference") (OtherActor :type "Actor Object Reference") (OtherComp :type "PrimitiveComponent Object Reference") (OtherBodyIndex :type Integer))
  (cast `/Game/GameBank/Blueprints/Characters/Player/Zone/BP_ThirdPersonCharacter` OtherActor)
  (`SceneComponent.SetVisibility` (`self.PostProcessToxic`) false false)
  (set `self.PlayerInside` false)
  (`/Game/GameBank/HUD/Widgets/Player/Zone/Damage/WBP_Hit.RemoveHitWidget` (`self.FeedbackWidget`))
  (goto _label_2 :!via `Reset`))

(fn `UserConstructionScript`)