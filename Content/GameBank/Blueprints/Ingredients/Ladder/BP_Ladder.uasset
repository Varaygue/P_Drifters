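; BP_Ladder is a ladder ingredient actor that moves the third-person character from its entry volume to its descend point.
; Overlap events on EnterCollision cache the BP_ThirdPersonCharacter and toggle a CanClimb flag.
; While the flag is set, Tick snaps the character to DescendCollision's world location without sweeping, so there is no gradual climbing movement or input check.
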(event `self.ReceiveTick`
  (params (DeltaSeconds :type "Float (single-precision)"))
  (if (`self.canClimb`)
    (`self.K2_SetActorLocation` (stale `self.EnterCollision.OnComponentBeginOverlap` _asbp_third_person_character) (`SceneComponent.K2_GetComponentLocation` (`self.DescendCollision`)) false false)))

(event `self.EnterCollision.OnComponentBeginOverlap`
  (params (OverlappedComponent :type "PrimitiveComponent Object Reference") (OtherActor :type "Actor Object Reference") (OtherComp :type "PrimitiveComponent Object Reference") (OtherBodyIndex :type Integer) (bFromSweep :type Boolean) (SweepResult :type "HitResult Structure (by ref)"))
  (bind _asbp_third_person_character (cast `/Game/GameBank/Blueprints/Characters/Player/Zone/BP_ThirdPersonCharacter` OtherActor))
  (set `self.canClimb` true))

(event `self.EnterCollision.OnComponentEndOverlap`
  (params (OverlappedComponent :type "PrimitiveComponent Object Reference") (OtherActor :type "Actor Object Reference") (OtherComp :type "PrimitiveComponent Object Reference") (OtherBodyIndex :type Integer))
  (cast `/Game/GameBank/Blueprints/Characters/Player/Zone/BP_ThirdPersonCharacter` OtherActor)
  (set `self.canClimb` false))

(fn `UserConstructionScript`)