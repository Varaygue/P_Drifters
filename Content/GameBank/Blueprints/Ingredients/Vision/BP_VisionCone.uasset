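; Vision cone actor that draws a flat procedural mesh of its line of sight, clipped by blocking geometry.
; Raycast fans Visibility traces across the vision arc, plus traces on a second channel that only print "Enemy" on a hit.
; HitTo2D converts hit or end points to local 2D polygon vertices for a dynamic mesh.
; Construction builds the mesh, and Tick re-triangulates it only when trace results change.
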(event `self.ReceiveBeginPlay`
  (bind _hitlocations (`self.Raycast`))
  (set `self.LastHitResults` _hitlocations))

(event `self.ReceiveTick`
  (params (DeltaSeconds :type "Float (single-precision)"))
  (bind _hitlocations (`self.Raycast`))
  (set `self.NewHitResults` _hitlocations)
  (if (not (`KismetArrayLibrary.Array_Identical` (`self.NewHitResults`) (`self.LastHitResults`)))
    (bind _returnvalue (`DynamicMesh.Reset` (`self.DynamicMesh`)))
    (bind _returnvalue_2 (`GeometryScriptLibrary_MeshPrimitiveFunctions.AppendTriangulatedPolygon` _returnvalue (struct) (struct) (`self.HitTo2D` (`self.NewHitResults`)) true null))
    (set `self.LastHitResults` (`self.NewHitResults`))
    (`KismetSystemLibrary.PrintString` (`KismetStringLibrary.Conv_IntToString` (`KismetArrayLibrary.Array_Length` (`self.NewHitResults`))) true true (struct :`G` 0.66 :`B` 1.0 :`A` 1.0) 0.0)))

(fn `HitTo2D`
  (params (HitResults :type "Array of HitResult Structure"))
  (returns (`2DVertices` :type "Array of Vector2D Structure"))
  (locals (LocalVector2D :type "Array of Vector2D Structure"))
  (`KismetArrayLibrary.Array_Add` (`local.LocalVector2D`))
  (for _array_element HitResults
    (bind (_bblockinghit _binitialoverlap _time _distance _location _impactpoint _normal _impactnormal _physmat _hitactor _hitcomponent _hitbonename _bonename _hititem _elementindex _faceindex _tracestart _traceend) (`GameplayStatics.BreakHitResult` _array_element))
    (`KismetArrayLibrary.Array_Add` (`local.LocalVector2D`) (`KismetMathLibrary.MakeVector2D` (.x (`KismetMathLibrary.InverseTransformLocation` (`self.GetTransform`) (`KismetMathLibrary.SelectVector` _location _traceend _bblockinghit))) (.y (`KismetMathLibrary.InverseTransformLocation` (`self.GetTransform`) (`KismetMathLibrary.SelectVector` _location _traceend _bblockinghit))))))
  (return (`local.LocalVector2D`)))

(fn `Raycast`
  (returns (HitLocations :type "Array of HitResult Structure"))
  (locals (HitResults :type "Array of HitResult Structure"))
  (bind _returnvalue (`self.K2_GetActorLocation`))
  (`|ExecutionSequence`
    (:`then_0`
      (for _index (range (+ (`KismetMathLibrary.FCeil` (/ (`self.VisionArc`) (`self.TestVisionArc`))) 1))
        (bind _returnvalue_2 (* _index (`self.TestVisionArc`)))
        (bind _returnvalue_3 (+ _returnvalue (`KismetMathLibrary.RotateAngleAxis` (* (`self.GetActorForwardVector`) (`self.VisionLength`)) (- (`KismetMathLibrary.FClamp` _returnvalue_2 _returnvalue_2 (`self.VisionArc`)) (/ (`self.VisionArc`) 2.0)) (0.0 0.0 1.0))))
        (bind _outhit (`KismetSystemLibrary.LineTraceSingle` _returnvalue _returnvalue_3 "TraceTypeQuery1"))
        (`KismetArrayLibrary.Array_Add` (`local.HitResults`) _outhit)
        (bind (_outhit_2 _returnvalue_4) (`KismetSystemLibrary.LineTraceSingle` _returnvalue _returnvalue_3 "TraceTypeQuery7"))
        (if _returnvalue_4
          (`KismetSystemLibrary.PrintString` "Enemy")))
      (return (`local.HitResults`)))))

(fn `UserConstructionScript`
  (`|ExecutionSequence`
    (:`then_0`
      (bind _returnvalue (`AddComponent|NODE_AddDynamicMeshComponent-0`))
      (bind _output_get (set `self.DMC` _returnvalue))
      (bind _returnvalue_2 (`BaseDynamicMeshComponent.GetDynamicMesh` _output_get))
      (set `self.DynamicMesh` _returnvalue_2))
    (:`then_1`
      (bind _hitlocations (`self.Raycast`))
      (`GeometryScriptLibrary_MeshPrimitiveFunctions.AppendTriangulatedPolygon` (`self.DynamicMesh`) (struct) (struct) (`self.HitTo2D` _hitlocations) true null)
      (`PrimitiveComponent.SetMaterial` (`self.DMC`) 0 "/Engine/OpenWorldTemplate/LandscapeMaterial/M_ProcGrid.M_ProcGrid"))))