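; BP_PlayerWorld is a player actor with a zoomable camera, placed at a point of interest when play begins.
; BeginPlay finds a single BP_PointOfInterest, stores it in ZonePositions and moves the actor to the first entry's location.
; Mouse wheel input steps the camera diagonally along world X and Z, with limits checked against its relative location.
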(event `Key|MouseScrollUp`
  (params (Key :type "Key Structure"))
  (bind _camera (`self.Camera`))
  (bind (_returnvalue_x _returnvalue_y _returnvalue_z) (`KismetMathLibrary.BreakVector` (`SceneComponent.K2_GetComponentLocation` _camera)))
  (bind (_relativelocation_x _relativelocation_y _relativelocation_z) (`KismetMathLibrary.BreakVector` (`SceneComponent.RelativeLocation` (`self.Camera`))))
  (:`Pressed`
    (if (and (< _relativelocation_x -100.0) (> _relativelocation_z 100.0))
      (`SceneComponent.K2_SetWorldLocation` _camera (`KismetMathLibrary.MakeVector` (+ _returnvalue_x 100.0) _returnvalue_y (- _returnvalue_z 100.0)) false false))))

(event `Key|MouseScrollDown`
  (params (Key :type "Key Structure"))
  (bind _camera (`self.Camera`))
  (bind (_returnvalue_x _returnvalue_y _returnvalue_z) (`KismetMathLibrary.BreakVector` (`SceneComponent.K2_GetComponentLocation` _camera)))
  (bind (_relativelocation_x _relativelocation_y _relativelocation_z) (`KismetMathLibrary.BreakVector` (`SceneComponent.RelativeLocation` (`self.Camera`))))
  (:`Pressed`
    (if (and (> _relativelocation_x -2000.0) (< _relativelocation_z 2000.0))
      (`SceneComponent.K2_SetWorldLocation` _camera (`KismetMathLibrary.MakeVector` (- _returnvalue_x 100.0) _returnvalue_y (+ _returnvalue_z 100.0)) false false))))

(event `self.ReceiveBeginPlay`
  (bind _returnvalue (`GameplayStatics.GetActorOfClass` "/Game/GameBank/Blueprints/World/BP_PointOfInterest.BP_PointOfInterest_C"))
  (`KismetArrayLibrary.Array_Set` (`self.ZonePositions`) 0 _returnvalue)
  (`self.K2_SetActorLocation` (`self.K2_GetActorLocation` (`|GetArrayItem` (`self.ZonePositions`)))))

(event `self.ReceiveTick`
  (params (DeltaSeconds :type "Float (single-precision)")))

(fn `UserConstructionScript`)