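; GM_World is a game mode that sets up per-level save data and player input when play begins.
; It loads the SAVE_LevelData slot named after the current level, or creates a new save object if none exists, and keeps it in LevelSaveObject.
; It then switches the first player controller to Game and UI input mode.
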(event `self.ReceiveBeginPlay`
  (`self.InitLevelSaveData`)
  (`WidgetBlueprintLibrary.SetInputMode_GameAndUIEx` (`GameplayStatics.GetPlayerController` 0) null))

(fn `InitLevelSaveData`
  (bind _returnvalue (`GameplayStatics.GetCurrentLevelName` true))
  (bind _returnvalue_2 (`GameplayStatics.DoesSaveGameExist` _returnvalue))
  (if _returnvalue_2
    (bind _returnvalue_3 (`GameplayStatics.GetCurrentLevelName` true))
    (bind _returnvalue_4 (`GameplayStatics.LoadGameFromSlot` _returnvalue_3))
    (bind _assave_level_data (cast `/Game/GameBank/Blueprints/Ingredients/SaveSystem/SAVE_LevelData` _returnvalue_4))
    (set `self.LevelSaveObject` _assave_level_data)
    (else
      (bind _returnvalue_5 (`GameplayStatics.CreateSaveGameObject` "/Game/GameBank/Blueprints/Ingredients/SaveSystem/SAVE_LevelData.SAVE_LevelData_C"))
      (set `self.LevelSaveObject` _returnvalue_5))))

(fn `UserConstructionScript`)