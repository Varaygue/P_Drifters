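; BP_PointOfInterest is a clickable world location that the player jumps to.
; Clicking its StaticMesh moves the BP_PlayerWorld character straight to the actor's location without sweeping, then writes PlaceName into the player's CurrentLocation.
; Cursor-over events on the mesh show and hide HoverIndicator.
; A TokenMovement node is left unwired, so the move is instant.
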(event `self.StaticMesh.OnClicked`
  (params (TouchedComponent :type "PrimitiveComponent Object Reference") (ButtonPressed :type "Key Structure"))
  (bind _asbp_player_world (cast `/Game/ObjectBank/Blueprints/Player/BP_PlayerWorld` (`GameplayStatics.GetPlayerCharacter` 0)))
  (`self.K2_SetActorLocation` _asbp_player_world (`self.K2_GetActorLocation`) false false)
  (set `/Game/ObjectBank/Blueprints/Player/BP_PlayerWorld.CurrentLocation` (`self.PlaceName`) _asbp_player_world))

(event `self.StaticMesh.OnBeginCursorOver`
  (params (TouchedComponent :type "PrimitiveComponent Object Reference"))
  (`SceneComponent.SetVisibility` (`self.HoverIndicator`) true false))

(event `self.StaticMesh.OnEndCursorOver`
  (params (TouchedComponent :type "PrimitiveComponent Object Reference"))
  (`SceneComponent.SetVisibility` (`self.HoverIndicator`) false false))

(fn `UserConstructionScript`)